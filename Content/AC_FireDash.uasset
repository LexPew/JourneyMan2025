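; Actor component that gives the player's BP_Astro pawn a horizontal air dash, usable only while falling.
; ActivateDash cancels the jump, plays a sound and sets velocity along the pawn's horizontal forward vector, switching to Flying movement to hold height.
; After a short delay it restores Walking mode, then a further delay acts as a cooldown before the DashActive flag clears for another dash.
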(event Custom|ActivateDash
  (bind _astroref (Variables|Default|GetAstroRef))
  (bind _dashvelocity (Variables|Default|GetDashVelocity))
  (bind _returnvalue (Transformation|GetActorForwardVector _astroref))
  (bind _charactermovement (Variables|/Script/Engine.Character|GetCharacterMovement _astroref))
  (if (not (Variables|Default|GetDashActive?))
    (if (AI|Components|NavMovement|IsFalling _charactermovement)
      (Variables|Default|SetDashActive? true)
      (Character|StopJumping _astroref)
      (Audio|PlaySoundatLocation 0 (Transformation|GetActorLocation _astroref) "0, 0, 0" 1.0 1.0 0.0 0 0 0 0)
      (Pawn|Components|CharacterMovement|SetMovementMode _charactermovement "MOVE_Flying" 0)
      (Variables|/Script/Engine.MovementComponent|SetVelocity _charactermovement (Math|Vector|MakeVector (* (.x _returnvalue) _dashvelocity) (* (.y _returnvalue) _dashvelocity) 0.0))
      (Utilities|FlowControl|Delay 0.5)
      (Pawn|Components|CharacterMovement|SetMovementMode _charactermovement "MOVE_Walking" 0)
      (Utilities|FlowControl|Delay 1.0)
      (Variables|Default|SetDashActive? false))))

(event EventBeginPlay
  (bind _asbp_astro (Utilities|Casting|CastToBP_Astro (Game|Player|GetPlayerPawn 0)))
  (Variables|Default|SetAstroRef _asbp_astro))