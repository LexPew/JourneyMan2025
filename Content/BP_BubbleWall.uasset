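; BP_BubbleWall is a wall that the player's BP_Astro pawn can pass through only while its bubble is active.
; On BeginPlay it caches the player pawn as BP_Astro.
; Its collision box disables WallMesh collision when that pawn begins overlapping with BubbleActive set, and restores it to query-only when the overlap ends.
; The bubble state is checked only at the moment the overlap begins.
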(event OnComponentBeginOverlap(CollisionBox)
  (params (OverlappedComponent :type Primitive%20Component%20Object%20Reference) (OtherActor :type Actor%20Object%20Reference) (OtherComp :type Primitive%20Component%20Object%20Reference) (OtherBodyIndex :type Integer) (bFromSweep :type Boolean) (SweepResult :type Hit%20Result%20Structure%20%28by%20ref%29))
  (bind _astroref (Variables|Default|GetAstroRef))
  (if (== OtherActor _astroref)
    (if (Variables|/Game/Blueprints/Character/BP_Astro.BP_Astro_C|GetBubbleActive? _astroref)
      (Collision|SetCollisionEnabled (Variables|Default|GetWallMesh) "NoCollision"))))

(event OnComponentEndOverlap(CollisionBox)
  (params (OverlappedComponent :type Primitive%20Component%20Object%20Reference) (OtherActor :type Actor%20Object%20Reference) (OtherComp :type Primitive%20Component%20Object%20Reference) (OtherBodyIndex :type Integer))
  (if (== OtherActor (Variables|Default|GetAstroRef))
    (Collision|SetCollisionEnabled (Variables|Default|GetWallMesh) "QueryOnly")))

(event EventBeginPlay
  (bind _asbp_astro (Utilities|Casting|CastToBP_Astro (Game|Player|GetPlayerPawn 0)))
  (Variables|Default|SetAstroRef _asbp_astro))

(fn ConstructionScript)