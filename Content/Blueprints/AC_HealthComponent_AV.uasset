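; Actor component that tracks health and handles death with an explosion effect and player respawn.
; DamageCalculation prints the damage type's class name, subtracts damage from Health, and at zero or below sets IsDead and fires EventDeath.
; EventDeath spawns a scaled Niagara explosion at the owner's location, then after a short delay respawns the BP_Astro pawn cached on BeginPlay if the DyingActor check matches.
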(event Custom|EventDeath
  (params (DyingActor :type Actor%20Object%20Reference))
  (Niagara|SpawnSystematLocation "/Game/FX/Explosion/NS_Explosion_AV.NS_Explosion_AV" (Transformation|GetWorldLocation (Variables|/Script/Engine.Actor|GetRootComponent (Components|GetOwner))) "0, 0, 0" (Variables|Default|GetExplosionScale))
  (Utilities|FlowControl|Delay 0.8)
  (if (== DyingActor "/Game/Blueprints/Character/BP_Astro.BP_Astro")
    (Default|Respawn (stale EventBeginPlay _asbp_astro) "0, 0, 0")))

(event EventBeginPlay
  (bind _asbp_astro (Utilities|Casting|CastToBP_Astro (Game|Player|GetPlayerPawn 0))))

(fn DamageCalculation
  (params (Damage :type Float%20%28double-precision%29) (DamageType :type Damage%20Type%20Class%20Reference))
  (Utilities|FlowControl|Sequence
    (:then_0
      (Development|PrintString (Utilities|GetClassDisplayName DamageType)))
    (:then_1
      (bind _output_get (Variables|Default|SetHealth (- (Variables|Default|GetHealth) Damage)))
      (if (<= _output_get 0.0)
        (Variables|Default|SetisDead? true)
        (CallFunction|EventDeath)))))