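; BP_AISpawnArea is a placeable spawn area that creates a group of enemies when play begins.
; SpawnAI loops over the Enemies array and spawns a BP_EnemyBase for each entry at its location offset from the actor, adjusting for collisions but always spawning.
; Each enemy receives its entry's elemental type, or the shared UniversalElement when AllSameElement is set.
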(event EventBeginPlay
  (CallFunction|SpawnAI))

(fn ConstructionScript)

(fn SpawnAI
  (for _array_element (Variables|Default|GetEnemies)
    (LocalVariables|SetLocationToSpawn (+ (.Location (Utilities|Struct|BreakST_EnemyData _array_element)) (Transformation|GetActorLocation)))
    (LocalVariables|SetElementType (.Element (Utilities|Struct|BreakST_EnemyData _array_element)))
    (Game|SpawnActorfromClass "/Game/Blueprints/AI/Characters/BaseClasses/BP_EnemyBase.BP_EnemyBase_C" (Math|Transform|MakeTransform (LocalVariables|GetLocationToSpawn)) "AdjustIfPossibleButAlwaysSpawn" "MultiplyWithRoot" 0 (select (Variables|Default|GetAll%20Same%20Element?) (Variables|Default|GetUniversal%20Element) (LocalVariables|GetElementType)) 0)))