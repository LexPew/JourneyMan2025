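; AI spawn point that places BP_EnemyBase actors of a set ElementalType around itself.
; BeginPlay spawns an initial batch, then optionally loops a timer, its interval randomized once, until MaxEnemiesToSpawn, which excludes that batch.
; SpawnWithinRadius re-rolls X/Y offsets against the radius, and FindZ line-traces downward for height; a reachable-point alternative is unconnected.
; The construction script sizes the radius decal and positions the trace-height marker.
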(event EventBeginPlay
  ;[1 1 1] Change to be "When activated"
  (CallFunction|InitialSpawn)
  (if (Variables|Editable|GetRepeatedly%20Spawn?)
    (Utilities|Time|SetTimerbyFunctionName 0 "SpawnAI" (Math|Random|RandomFloatinRange (Variables|Editable|GetSpawnFrequencyMin) (Variables|Editable|GetSpawnFrequencyMax)) true)))

(fn ConstructionScript
  (OnConstruct|CalculateCircleDecalSize)
  (OnConstruct|SetLineTraceHeightRef))

(fn InitialSpawn
  (for _index (range 0 (- (Variables|Editable|GetInitialSpawnAmount) 1))
    (bind _spawnlocation (CallFunction|SpawnWithinRadius))
    (Game|SpawnActorfromClass "/Game/Blueprints/AI/Characters/BaseClasses/BP_EnemyBase.BP_EnemyBase_C" (Math|Transform|MakeTransform _spawnlocation "0, 0, 0" "1.000000,1.000000,1.000000") "AdjustIfPossibleButAlwaysSpawn" "MultiplyWithRoot" 0 (Variables|Editable|GetElemental%20Type) 0)))

(fn SpawnAI
  (if (not (>= (Variables|Editable|GetAmountSpawned) (Variables|Editable|GetMaxEnemiesToSpawn)))
    (bind _spawnlocation (CallFunction|SpawnWithinRadius))
    (Game|SpawnActorfromClass "/Game/Blueprints/AI/Characters/BaseClasses/BP_EnemyBase.BP_EnemyBase_C" (Math|Transform|MakeTransform _spawnlocation "0, 0, 0" "1.000000,1.000000,1.000000") "AdjustIfPossibleButAlwaysSpawn" "MultiplyWithRoot" 0 (Variables|Editable|GetElemental%20Type) 0)
    (Math|Integer|IncrementInt (Variables|Editable|GetAmountSpawned))))

(fn CalculateCircleDecalSize
  (bind _spawnrange__radius_ (Variables|Editable|GetSpawnRange%20%28Radius%29))
  (bind _returnvalue (/ _spawnrange__radius_ 2.5e+02))
  (Transformation|SetWorldScale3D (Variables|Default|GetDecal) (Math|Vector|MakeVector 0.1 _returnvalue _returnvalue)))

(fn FindZ
  (params (RandX :type Float%20%28double-precision%29) (RandY :type Float%20%28double-precision%29))
  (bind _outhit (Collision|LineTraceByChannel (Math|Vector|MakeVector RandX RandY (Variables|Editable|GetLineTraceStartZHeight)) (Math|Vector|MakeVector RandX RandY -1e+03) "TraceTypeQuery1" false 0 "Persistent"))
  (if (!= (Utilities|GetClass (.hitactor _outhit)) "/Script/Engine.Character")
    (return (.Z (Math|Vector|BreakVector (.location _outhit))))))

(fn SetLineTraceHeightRef
  (bind _linetraceheightref (Variables|Default|GetLineTraceHeightRef))
  (bind _returnvalue (Transformation|GetWorldLocation _linetraceheightref))
  (Transformation|SetWorldLocation _linetraceheightref (Math|Vector|MakeVector (.x _returnvalue) (.y _returnvalue) (Variables|Editable|GetLineTraceStartZHeight)) false false))

(fn SpawnWithinRadius
  (bind _rand (Utilities|RandomLocationWithinRange))
  (bind _rand_2 (Utilities|RandomLocationWithinRange))
  ;[0 1 0] Current Method
  (LocalVariables|SetRandX _rand_2)
  (LocalVariables|SetRandY _rand)
  (while (> (Math|Float|Absolute(Float) (Math|Vector|Distance(Vector) (Transformation|GetActorLocation) (Math|Vector|MakeVector (.x (+ (Transformation|GetActorLocation) (Math|Vector|MakeVector (LocalVariables|GetRandX) (LocalVariables|GetRandY) 0.0))) (.y (+ (Transformation|GetActorLocation) (Math|Vector|MakeVector (LocalVariables|GetRandX) (LocalVariables|GetRandY) 0.0))) 0.0))) (Variables|Editable|GetSpawnRange%20%28Radius%29))
    (LocalVariables|SetRandX _rand_2)
    (LocalVariables|SetRandY _rand))
  (bind _z (CallFunction|FindZ (.x (+ (Transformation|GetActorLocation) (Math|Vector|MakeVector (LocalVariables|GetRandX) (LocalVariables|GetRandY) 0.0))) (.y (+ (Transformation|GetActorLocation) (Math|Vector|MakeVector (LocalVariables|GetRandX) (LocalVariables|GetRandY) 0.0)))))
  (return (Math|Vector|MakeVector (.X (Math|Vector|BreakVector (Math|Vector|MakeVector (.x (+ (Transformation|GetActorLocation) (Math|Vector|MakeVector (LocalVariables|GetRandX) (LocalVariables|GetRandY) 0.0))) (.y (+ (Transformation|GetActorLocation) (Math|Vector|MakeVector (LocalVariables|GetRandX) (LocalVariables|GetRandY) 0.0))) 0.0))) (.Y (Math|Vector|BreakVector (Math|Vector|MakeVector (.x (+ (Transformation|GetActorLocation) (Math|Vector|MakeVector (LocalVariables|GetRandX) (LocalVariables|GetRandY) 0.0))) (.y (+ (Transformation|GetActorLocation) (Math|Vector|MakeVector (LocalVariables|GetRandX) (LocalVariables|GetRandY) 0.0))) 0.0))) _z)))