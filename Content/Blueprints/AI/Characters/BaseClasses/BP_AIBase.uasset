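; Base AI character Blueprint with an elemental type that determines its mannequin's look.
; The construction script switches on ElementalType to assign both mesh material slots a color set for Neutral, Air, Fire, Water or Earth.
; Health query, heal and damage functions are stubs returning zero or false, and BeginPlay does nothing.
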(event EventBeginPlay)

(fn ConstructionScript
  (bind _mesh (Variables|Character|GetMesh))
  (Utilities|FlowControl|Sequence
    (:then_0
      (switch Utilities|FlowControl|Switch|SwitchonE_ElementalType (Variables|Stats|GetElemental%20Type)
        (:NewEnumerator0
          (Rendering|Material|SetMaterial _mesh 0 "/Game/Blueprints/AI/TempMaterials/M_MannyBlack0.M_MannyBlack0")
          (Rendering|Material|SetMaterial _mesh 1 "/Game/Blueprints/AI/TempMaterials/M_MannyBlack1.M_MannyBlack1"))
        (:NewEnumerator1
          (Rendering|Material|SetMaterial _mesh 0 "/Game/Blueprints/AI/TempMaterials/M_MannyWhite0.M_MannyWhite0")
          (Rendering|Material|SetMaterial _mesh 1 "/Game/Blueprints/AI/TempMaterials/M_MannyWhite1.M_MannyWhite1"))
        (:NewEnumerator2
          (Rendering|Material|SetMaterial _mesh 0 "/Game/Blueprints/AI/TempMaterials/M_MannyRed0.M_MannyRed0")
          (Rendering|Material|SetMaterial _mesh 1 "/Game/Blueprints/AI/TempMaterials/M_MannyRed1.M_MannyRed1"))
        (:NewEnumerator3
          (Rendering|Material|SetMaterial _mesh 0 "/Game/Blueprints/AI/TempMaterials/M_MannyBlue0.M_MannyBlue0")
          (Rendering|Material|SetMaterial _mesh 1 "/Game/Blueprints/AI/TempMaterials/M_MannyBlue1.M_MannyBlue1"))
        (:NewEnumerator4
          (Rendering|Material|SetMaterial _mesh 0 "/Game/Blueprints/AI/TempMaterials/M_MannyGreen0.M_MannyGreen0")
          (Rendering|Material|SetMaterial _mesh 1 "/Game/Blueprints/AI/TempMaterials/M_MannyGreen1.M_MannyGreen1"))))))

(fn GetCurrentHealth
  (return 0.0))

(fn GetMaxHealth
  (return 0.0))

(fn Heal
  (params (Amount :type Float%20%28double-precision%29))
  (return 0.0))

(fn Takedamage
  (params (Damageinfo :type S%20D%20Amage%20Info%20Structure))
  (return false))