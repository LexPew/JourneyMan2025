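; Base enemy character that feeds its task and player sightings to an AI blackboard, forgetting the target five seconds after last sight.
; Attack chooses by range between a melee sphere trace and an elemental shot: predictive arcing fire, homing water or scattered rocks, with timer-driven facing for ranged.
; Attack hits switch the mesh to physics and launch it; striking flat ground spawns fire effects, then destroys the actor.
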(event OnSeePawn(PawnSensing)
  (params (Pawn :type Pawn%20Object%20Reference))
  (Utilities|FlowControl|Sequence
    (:then_0
      ;[1 1 1] Change bool if lost target
      (Utilities|FlowControl|RetriggerableDelay 5.0)
      (AI|Components|Blackboard|SetValueasBool (AI|GetBlackboard (AI|GetAIController self)) (Utilities|Name|MakeLiteralName "SeenPlayer?") false)
      (Variables|Default|SetTarget 0))
    (:then_1
      (AI|Components|Blackboard|SetValueasBool (AI|GetBlackboard (AI|GetAIController self)) (Utilities|Name|MakeLiteralName "SeenPlayer?") true)
      (Variables|Default|SetTarget Pawn))))

(event OnComponentHit(Mesh)
  (params (HitComponent :type Primitive%20Component%20Object%20Reference) (OtherActor :type Actor%20Object%20Reference) (OtherComp :type Primitive%20Component%20Object%20Reference) (NormalImpulse :type Vector :default "0, 0, 0") (Hit :type Hit%20Result%20Structure%20%28by%20ref%29))
  (bind _impactnormal (Collision|BreakHitResult Hit))
  (bind _self self)
  (bind _z (Math|Vector|BreakVector _impactnormal))
  (if (and (>= _z 0.99) (< _z 1.01))
    (Niagara|SpawnSystematLocation "/Game/FX/FireDash/NS_Fire.NS_Fire" (Transformation|GetActorLocation _self))
    (Utilities|FlowControl|Delay 0.2)
    (Actor|DestroyActor _self)))

(event EventBeginPlay
  ;[1 1 1] Assign Task
  (AI|Components|Blackboard|SetValueasEnum (AI|GetBlackboard (AI|GetAIController self)) (Utilities|Name|MakeLiteralName "DefaultTask") (Utilities|Select :Index (Variables|Default|GetTask) :NewEnumerator0 0 :NewEnumerator1 0)))

(event EventOnAttackHit
  (params (AttackingPlayer :type Character%20Object%20Reference) (KnockbackStrength :type Float%20%28double-precision%29))
  (bind _self self)
  (bind _mesh (Variables|Character|GetMesh _self))
  (Components|Movement|StopMovementImmediately (Variables|Character|GetCharacterMovement _self))
  (Physics|SetSimulatePhysics _mesh true)
  (Collision|SetCollisionEnabled _mesh "PhysicsOnly")
  (Physics|AddImpulse (Variables|Character|GetMesh _self) (+ (* KnockbackStrength (Transformation|GetActorForwardVector AttackingPlayer)) (Math|Vector|MakeVector 0.0 0.0 (* KnockbackStrength 0.75))) "None" true))

(fn ConstructionScript
  (|CallParentFunction))

(fn Attack
  (bind _returnvalue (Transformation|GetActorLocation))
  (bind _meleerange (Variables|Combat|GetMeleeRange))
  (bind _target (Variables|Default|GetTarget))
  (bind _returnvalue_2 (Transformation|GetActorLocation _target))
  (bind _returnvalue_3 (Math|Vector|Distance(Vector) _returnvalue _returnvalue_2))
  (bind _returnvalue_4 (>= _returnvalue_3 _meleerange))
  (Utilities|IsValid _target
    (:Is%20Valid
      ;[1 1 1] Melee or ranged?
      (if _returnvalue_4
        (Utilities|Time|SetTimerbyFunctionName 0 "LockRotation" 0.1 _returnvalue_4)
        (switch Utilities|FlowControl|Switch|SwitchonE_ElementalType (Variables|Default|GetElemental%20Type)
          (:NewEnumerator2
            (CallFunction|FireShot))
          (:NewEnumerator3
            (CallFunction|WaterShot))
          (:NewEnumerator4
            (CallFunction|EarthShot)))
        (else
          (CallFunction|Melee))))))

(fn FireShot
  (Utilities|IsValid (Variables|Default|GetTarget)
    (:Is%20Valid
      (bind _predicted_location (CallFunction|PredictTargetDirection (Variables|Default|GetTarget)))
      (bind (_outlaunchvelocity _returnvalue) (Game|SuggestProjectileVelocityCustomArc (Transformation|GetWorldLocation (Variables|Default|GetProjectileStartPoint)) _predicted_location 0.0 0.5))
      (if _returnvalue
        (bind _returnvalue_2 (Game|SpawnActorfromClass "/Game/Blueprints/AI/Projectiles/BP_FireShot.BP_FireShot_C" (Math|Transform|MakeTransform (Transformation|GetWorldLocation (Variables|Default|GetProjectileStartPoint)) "0, 0, 0" "1.000000,1.000000,1.000000") "Undefined" "MultiplyWithRoot" 0 0))
        (Utilities|IsValid _returnvalue_2
          (:Is%20Valid
            (Game|Components|ProjectileMovement|SetVelocityinLocalSpace (Variables|/Game/Blueprints/AI/Projectiles/BP_ProjectileBase.BP_ProjectileBase_C|GetProjectileMovement _returnvalue_2) _outlaunchvelocity)))))))

(fn PredictTargetDirection
  (params (TargetActor :type Actor%20Object%20Reference))
  (LocalVariables|SetTargetActorVelocity (Transformation|GetVelocity TargetActor))
  (LocalVariables|SetTargetActorLocation (Transformation|GetActorLocation TargetActor))
  (Rendering|Debug|DrawDebugSphere (+ (LocalVariables|GetTargetActorLocation) (* (LocalVariables|GetTargetActorVelocity) (/ (Math|Vector|Distance(Vector) (LocalVariables|GetTargetActorLocation) (Transformation|GetActorLocation)) (Math|Float|MakeLiteralFloat 5e+02)))) 1e+01 4 "(R=0.059655,G=1.000000,B=0.000000,A=1.000000)" 2.0 2.0)
  (return (+ (LocalVariables|GetTargetActorLocation) (* (LocalVariables|GetTargetActorVelocity) (/ (Math|Vector|Distance(Vector) (LocalVariables|GetTargetActorLocation) (Transformation|GetActorLocation)) (Math|Float|MakeLiteralFloat 5e+02))))))

(fn WaterShot
  (Game|SpawnActorfromClass "/Game/Blueprints/AI/Projectiles/BP_WaterShot.BP_WaterShot_C" (Transformation|GetWorldTransform (Variables|Default|GetProjectileStartPoint)) "Undefined" "MultiplyWithRoot" 0 (Variables|/Script/Engine.Actor|GetRootComponent (Variables|Default|GetTarget)) 0 self))

(fn Melee
  (Collision|SphereTraceByChannel (Transformation|GetActorLocation) (+ (Transformation|GetActorLocation) (* (Math|Vector|GetForwardVector (Math|Rotator|FindLookatRotation (Transformation|GetActorLocation) (Transformation|GetActorLocation (Variables|Default|GetTarget)))) (Variables|Combat|GetMeleeRange))) 5e+01 "TraceTypeQuery1" false 0 "ForDuration")
  (CallFunction|Takedamage (Utilities|Struct|MakeS_DAmageInfo (Variables|Combat|GetMeleeDamage) "NewEnumerator1" "NewEnumerator1" false true true false)))

(fn LockRotation
  (bind _returnvalue (Transformation|GetActorLocation))
  (bind _target (Variables|Default|GetTarget))
  (bind _returnvalue_2 (Transformation|GetActorLocation _target))
  (bind _returnvalue_3 (Math|Rotator|FindLookatRotation _returnvalue _returnvalue_2))
  (Utilities|IsValid _target
    (:Is%20Valid
      (Transformation|SetActorRotation (Math|Rotator|MakeRotator (.roll _returnvalue_3) 0.0 (.yaw _returnvalue_3))))))

(fn EarthShot
  (bind _returnvalue (Transformation|GetActorLocation))
  (bind _target (Variables|Default|GetTarget))
  (bind _returnvalue_2 (Transformation|GetActorLocation _target))
  (bind _returnvalue_3 (Math|Rotator|FindLookatRotation _returnvalue _returnvalue_2))
  (for _index (range 1 (LocalVariables|GetRockAmount%20))
    (Game|SpawnActorfromClass "/Game/Blueprints/AI/Projectiles/BP_EarthShot.BP_EarthShot_C" (Math|Transform|MakeTransform (Transformation|GetWorldLocation (Variables|Default|GetProjectileStartPoint)) (Math|Rotator|MakeRotator (+ (.roll _returnvalue_3) (Math|Random|RandomFloatinRange -5.0 5.0)) (+ (.pitch _returnvalue_3) (Math|Random|RandomFloatinRange -5.0 5.0)) (+ (.yaw _returnvalue_3) (Math|Random|RandomFloatinRange -5.0 5.0))) "1.000000,1.000000,1.000000") "Undefined" "MultiplyWithRoot" 0 0)))

(fn IsAttackable
  (return false))