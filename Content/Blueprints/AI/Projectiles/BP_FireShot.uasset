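; AI fire projectile that kills BP_Astro actors near its impact point and runs the inherited velocity check each tick.
; Mesh collision switches on after a short delay from BeginPlay.
; The first hit passing a class filter (excludes other fire shots) runs a debug-drawn sphere trace, calling EventDeath on Astros found.
; The shot destroys itself only when that trace finds an Astro.
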(event EventBeginPlay
  (Utilities|FlowControl|Delay 0.2)
  (Collision|SetCollisionEnabled (Variables|Default|GetProjectileMesh) "QueryAndPhysics"))

(event Collision|EventHit
  (params (MyComp :type Primitive%20Component%20Object%20Reference) (Other :type Actor%20Object%20Reference) (OtherComp :type Primitive%20Component%20Object%20Reference) (bSelfMoved :type Boolean) (HitLocation :type Vector :default "0, 0, 0") (HitNormal :type Vector :default "0, 0, 0") (NormalImpulse :type Vector :default "0, 0, 0") (Hit :type Hit%20Result%20Structure%20%28by%20ref%29))
  (if (not (or (== (Utilities|GetClass Other) (Utilities|GetClass self)) (== (Utilities|GetClass (Game|GetInstigator Other)) (Utilities|GetClass Other))))
    (Utilities|FlowControl|DoOnce false
      (:Completed
        (Development|PrintString "Hello")
        (bind _outhits (Collision|MultiSphereTraceByChannel HitLocation HitLocation 2e+02 "TraceTypeQuery1" false 0 "ForDuration"))
        (bind _array_element (Utilities|Array|ForEachLoopwithBreak _outhits)
          (:LoopBody
            (bind _asbp_astro (Utilities|Casting|CastToBP_Astro (.HitActor (Collision|BreakHitResult _array_element))))
            (Default|EventDeath _asbp_astro)
            (Actor|DestroyActor)))))))

(event EventTick
  (params (DeltaSeconds :type Float%20%28single-precision%29))
  (|CallParentFunction DeltaSeconds)
  (CallFunction|VelocityCheck))

(fn ConstructionScript
  (|CallParentFunction))