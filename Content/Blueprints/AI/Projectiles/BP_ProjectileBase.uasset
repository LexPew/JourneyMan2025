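; BP_ProjectileBase is a base projectile actor for AI that destroys itself ten seconds after BeginPlay.
; A VelocityCheck event would destroy it when it nearly stops, but the looping timer that would call it is disconnected and never runs.
; Its health, heal and damage functions are stubs that return zero or false, so the projectile has no health and reports no damage taken.
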(event Custom|Velocity%20Check
  (if (< (Math|Vector|VectorLength (Transformation|GetVelocity)) 5.0)
    (Actor|DestroyActor)))

(event EventBeginPlay
  (Utilities|FlowControl|Delay 1e+01)
  (Actor|DestroyActor))

(fn ConstructionScript)

(fn GetCurrentHealth
  (return 0.0))

(fn GetMaxHealth
  (return 0.0))

(fn Heal
  (params (Amount :type Float%20%28double-precision%29))
  (return 0.0))

(fn Takedamage
  (params (Damageinfo :type S%20D%20Amage%20Info%20Structure))
  (return false))