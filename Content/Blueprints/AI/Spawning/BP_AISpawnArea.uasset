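; BP_AISpawnArea is a placeable spawner that creates a batch of BP_EnemyBase enemies at offsets from its own location.
; SpawnAI loops over the Enemies array, passing each entry's task and elemental type, with an option to give all enemies one shared element.
; It spawns immediately on BeginPlay, or, when SpawnCondition is set, polls on a looping timer until EnableSpawner is called, then spawns once and pauses the timer.
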(event Custom|CanSpawnCheck
  (if (Variables|Default|GetEnabled?)
    (CallFunction|SpawnAI)
    (Utilities|Time|PauseTimerbyHandle (stale EventBeginPlay _returnvalue))))

(event EventEnableSpawner
  (Variables|Default|SetEnabled? true))

(event EventBeginPlay
  (if (Variables|Default|GetSpawn%20Condition?)
    (bind _returnvalue (Utilities|Time|SetTimerbyEvent (delegate Custom|CanSpawnCheck) 0.1 true))
    (else
      (CallFunction|SpawnAI))))

(fn ConstructionScript)

(fn SpawnAI
  (for _array_element (Variables|Default|GetEnemies)
    (LocalVariables|SetLocationToSpawn (+ (.Location (Utilities|Struct|BreakST_EnemyData _array_element)) (Transformation|GetActorLocation)))
    (LocalVariables|SetElementType (.Element (Utilities|Struct|BreakST_EnemyData _array_element)))
    (LocalVariables|SetTask (.Task (Utilities|Struct|BreakST_EnemyData _array_element)))
    (Game|SpawnActorfromClass "/Game/Blueprints/AI/Characters/BaseClasses/BP_EnemyBase.BP_EnemyBase_C" (Math|Transform|MakeTransform (LocalVariables|GetLocationToSpawn)) "AdjustIfPossibleButAlwaysSpawn" "MultiplyWithRoot" 0 (LocalVariables|GetTask) (select (Variables|Default|GetAll%20Same%20Element?) (Variables|Default|GetUniversal%20Element) (LocalVariables|GetElementType)) 0)))