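; BP_AstroAirMerge is a playable character Blueprint with Enhanced Input movement, camera look, jump and a hold-to-activate air bubble.
; BeginPlay adds the IMC_Character mapping context, and movement follows the camera's forward and right vectors.
; Holding the bubble input shows BubbleMesh and sets the BubbleActive flag, which nothing here reads.
; The hover events and UpdateJumpOffset are unimplemented stubs.
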(event Input|EnhancedActionEvents|EnhancedInputActionIA_Move
  (params (ActionValue :type Vector%202D%20Structure) (ElapsedSeconds :type Float%20%28double-precision%29) (TriggeredSeconds :type Float%20%28double-precision%29) (InputAction :type Input%20Action%20Object%20Reference :default "/Game/Blueprints/Character/Inputs/IA_Move.IA_Move"))
  ;[1 1 1] Movement
  ;;[1 1 1] Add Forward / Back Movement
  (Pawn|Input|AddMovementInput (* (.y ActionValue) (Math|Vector|GetForwardVector (Variables|Default|GetCamera))) 1.0 false)
  ;;[1 1 1] Add Forward / Back Movement
  (Pawn|Input|AddMovementInput (* (.x ActionValue) (Math|Vector|GetRightVector (Variables|Default|GetCamera))) 1.0 false))

(event Input|EnhancedActionEvents|EnhancedInputActionIA_Look
  (params (ActionValue :type Vector%202D%20Structure) (ElapsedSeconds :type Float%20%28double-precision%29) (TriggeredSeconds :type Float%20%28double-precision%29) (InputAction :type Input%20Action%20Object%20Reference :default "/Game/Blueprints/Character/Inputs/IA_Look.IA_Look"))
  ;[1 1 1] Camera Controls
  (Pawn|Input|AddControllerPitchInput (.y ActionValue))
  (Pawn|Input|AddControllerYawInput (.x ActionValue)))

(event Input|EnhancedActionEvents|EnhancedInputActionIA_Jump
  (params (ActionValue :type Boolean) (ElapsedSeconds :type Float%20%28double-precision%29) (TriggeredSeconds :type Float%20%28double-precision%29) (InputAction :type Input%20Action%20Object%20Reference :default "/Game/Blueprints/Character/Inputs/IA_Jump.IA_Jump"))
  (:Started
    (Character|Jump))
  (:Completed
    (Character|StopJumping)))

(event Input|EnhancedActionEvents|EnhancedInputActionIA_ActivateBubble
  (params (ActionValue :type Boolean) (ElapsedSeconds :type Float%20%28double-precision%29) (TriggeredSeconds :type Float%20%28double-precision%29) (InputAction :type Input%20Action%20Object%20Reference :default "/Game/Blueprints/Character/Inputs/IA_ActivateBubble.IA_ActivateBubble"))
  (bind _bubblemesh (Variables|Default|GetBubbleMesh))
  (:Started
    (Rendering|SetVisibility _bubblemesh true false)
    (Variables|Default|SetBubbleActive? true))
  (:Completed
    (Rendering|SetVisibility _bubblemesh false false)
    (Variables|Default|SetBubbleActive? false)))

(event EventBeginPlay
  ;[1 1 1] Adds the Input Mapping Context
  (bind _asplayer_controller (Utilities|Casting|CastToPlayerController (Pawn|GetController)))
  (Utilities|IsValid (PlayerController|LocalPlayerSubsystems|GetEnhancedInputLocalPlayerSubsystem _asplayer_controller)
    (:Is%20Valid
      (Input|AddMappingContext (PlayerController|LocalPlayerSubsystems|GetEnhancedInputLocalPlayerSubsystem _asplayer_controller) "/Game/Blueprints/Character/Inputs/IMC_Character.IMC_Character" 0 "(bIgnoreAllPressedKeysUntilRelease=True,bForceImmediately=False,bNotifyUserSettings=False)"))))

(event Collision|EventActorBeginOverlap
  (params (OtherActor :type Actor%20Object%20Reference)))

(event EventTick
  (params (DeltaSeconds :type Float%20%28single-precision%29)))

(event EventOnStartHover)

(event EventOnStopHover)

(event Input|KeyboardEvents|SpaceBar
  (params (Key :type Key%20Structure)))

(fn ConstructionScript)