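; Appa is a one-time rideable mount that carries the player along a spline.
; It appears and disappears by player proximity with scale timelines and a wind burst, staying visible while ridden.
; Its trigger attaches the player, disables input and blends the camera, then a timeline drives the ride until dismount at DismountPoint.
; Banking comes from spline tangent change, smoothed on Tick alongside a sine hover bob, and construction snaps Appa to the spline start.
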(event OnComponentBeginOverlap(AppearDissapearDistance)
  (params (OverlappedComponent :type Primitive%20Component%20Object%20Reference) (OtherActor :type Actor%20Object%20Reference) (OtherComp :type Primitive%20Component%20Object%20Reference) (OtherBodyIndex :type Integer) (bFromSweep :type Boolean) (SweepResult :type Hit%20Result%20Structure%20%28by%20ref%29))
  ;[1 1 1] Appear On Enter Area
  (if (and (== OtherActor (Game|Player|GetPlayerPawn 0)) (Variables|HideShow|GetInvisible))
    (CallFunction|Appear)))

(event OnComponentBeginOverlap(TriggerBox)
  (params (OverlappedComponent :type Primitive%20Component%20Object%20Reference) (OtherActor :type Actor%20Object%20Reference) (OtherComp :type Primitive%20Component%20Object%20Reference) (OtherBodyIndex :type Integer) (bFromSweep :type Boolean) (SweepResult :type Hit%20Result%20Structure%20%28by%20ref%29))
  (bind _returnvalue (Game|Player|GetPlayerPawn 0))
  ;[1 1 1] Begin Spline Movement
  (if (and (== OtherActor _returnvalue) (not (Variables|HideShow|GetHasRode)))
    (bind _asbp_astro (Utilities|Casting|CastToBP_Astro _returnvalue))
    (Default|OnAppa _asbp_astro true)
    (Variables|Default|SetIsRiding true)
    (CallFunction|TransitionCamera self)
    (CallFunction|AttachPlayertoAppa)
    (CallFunction|StartSplineMovement)))

(event OnComponentEndOverlap(AppearDissapearDistance)
  (params (OverlappedComponent :type Primitive%20Component%20Object%20Reference) (OtherActor :type Actor%20Object%20Reference) (OtherComp :type Primitive%20Component%20Object%20Reference) (OtherBodyIndex :type Integer))
  (if (and (and (not (Variables|HideShow|GetInvisible)) (== OtherActor (Game|Player|GetPlayerPawn 0))) (== (Variables|Default|GetIsRiding) false))
    (CallFunction|Dissapear)))

(event Custom|StartSplineMovement
  ;[1 1 1] Begin Follow Timeline
  (Components|Timeline|SetPlayRate (Variables|Default|GetTimeline) (/ 1.0 (Variables|Spline|GetDuration)))
  (bind _movement (Timeline|Timeline PlayFromStart)
    (:Update
      (bind _returnvalue (CallFunction|ApplyActorRotationBasedonSplinePoint _movement))
      (CallFunction|CalculateandApplyRoll _returnvalue))
    (:Finished
      (Variables|HideShow|SetHasRode true)
      (Variables|Roll|SetRollAngle 0.0)
      (CallFunction|DetachPlayer)
      (CallFunction|TransitionCamera (Game|Player|GetPlayerPawn 0))
      (Variables|Default|SetIsRiding false)
      (bind _asbp_astro (Utilities|Casting|CastToBP_Astro (Game|Player|GetPlayerPawn 0)))
      (Default|OnAppa _asbp_astro false))))

(event Custom|Appear
  ;[1 1 1] Appear Logic
  (Variables|HideShow|SetInvisible false)
  (Rendering|SetVisibility (Variables|Default|GetAppa) true false)
  (Niagara|ResetSystem (Variables|Default|GetNS_WindBurst))
  (Components|Timeline|SetPlayRate (Variables|Default|GetScaleTimeLineUp) (/ 1.0 (Variables|Default|GetAppearDissappearDuration)))
  (bind _ftrack1 (Timeline|ScaleTimeLineUp PlayFromStart)
    (:Update
      (Transformation|SetWorldScale3D (Variables|Default|GetAppa) (Math|Conversions|ToVector(Float) _ftrack1)))))

(event Custom|Dissapear
  ;[1 1 1] Disappear Logic
  (Variables|HideShow|SetInvisible true)
  (Rendering|SetVisibility (Variables|Default|GetAppa) false false)
  (Niagara|ResetSystem (Variables|Default|GetNS_WindBurst))
  (Components|Timeline|SetPlayRate (Variables|Default|GetScaleTimeLineDown) (/ 1.0 (Variables|Default|GetAppearDissappearDuration)))
  (bind _newtrack_0 (Timeline|ScaleTimeLineDown ReverseFromEnd)
    (:Update
      (Transformation|SetWorldScale3D (Variables|Default|GetAppa) (Math|Conversions|ToVector(Float) _newtrack_0)))))

(event EventBeginPlay
  (CallFunction|Dissapear))

(event Collision|EventActorBeginOverlap
  (params (OtherActor :type Actor%20Object%20Reference)))

(event EventTick
  (params (DeltaSeconds :type Float%20%28single-precision%29))
  ;[1 1 1] Apply Smoothed Roll
  (CallFunction|ApplyRoll DeltaSeconds)
  ;[1 1 1] Hover up and down
  (CallFunction|HoverBob))

(fn ConstructionScript
  (CallFunction|CSetAppaonSplinePoint))

(fn AttachPlayertoAppa
  (bind _returnvalue (Game|Player|GetPlayerPawn 0))
  (bind _returnvalue_2 (Pawn|GetMovementComponent _returnvalue))
  (bind _ascharacter_movement_component (Utilities|Casting|CastToCharacterMovementComponent _returnvalue_2))
  (Components|Movement|StopMovementImmediately _returnvalue_2)
  (Input|DisableInput (Game|Player|GetPlayerPawn 0) (Game|GetPlayerController 0))
  (Pawn|Components|CharacterMovement|SetMovementMode _ascharacter_movement_component "MOVE_None" 0)
  (Collision|SetActorEnableCollision (Game|Player|GetPlayerPawn 0) false)
  (Transformation|AttachComponentToComponent (Game|Player|GetPlayerPawn 0) (Variables|Default|GetMountPoint) "None" "SnapToTarget" "SnapToTarget" "KeepWorld" true)
  (CallFunction|TransitionCamera self))

(fn TransitionCamera
  (params (NewViewTarget :type Actor%20Object%20Reference))
  (Game|Player|SetViewTargetwithBlend (Game|GetPlayerController 0) NewViewTarget (Variables|Camera|GetCameraBlendTime) "VTBlend_EaseInOut" 2.0 true))

(fn ApplyRoll
  (params (DeltaTime :type Float%20%28double-precision%29))
  (Transformation|SetRelativeRotation (Variables|Default|GetSplineMove_Root) (Math|Rotator|MakeRotator (Math|Interpolation|FInterpTo (.roll (Variables|/Script/Engine.SceneComponent|GetRelativeRotation (Variables|Default|GetSplineMove_Root))) (Variables|Roll|GetRollAngle) DeltaTime (Variables|Roll|GetRollSpeed)) 0.0 0.0) false false))

(fn HoverBob
  (bind _output_get (Variables|HoverBob|SetBobHeight (* (* (Math|Trig|Sin(Radians) (Actor|GetGameTimeSinceCreation)) (Variables|HoverBob|GetBobSpeed)) (Variables|HoverBob|GetBobAmp))))
  (Transformation|SetRelativeLocation (Variables|Default|GetSplineMove_Root) (Math|Vector|MakeVector 0.0 0.0 _output_get) false false))

(fn CalculateandApplyRoll
  (params (CurrentTangent :type Vector))
  ;[1 1 1] Calculates How Much Appa should rotate based on the curve
  (Variables|Spline|SetDeltaTangent (Math|Vector|Normalize (- CurrentTangent (Variables|Spline|GetPreviousTangent))))
  (Variables|Spline|SetPreviousTangent CurrentTangent)
  (Variables|Roll|SetRollAngle (* (* (.y (Variables|Spline|GetDeltaTangent)) (Variables|Roll|GetRollIntensity)) -1.0))
  (return))

(fn ApplyActorRotationBasedonSplinePoint
  (params (Alpha :type Float%20%28double-precision%29))
  (bind _returnvalue (Utilities|GetSplineIndex))
  (bind _spline (Variables|Default|GetSpline))
  (bind _returnvalue_2 (Math|Float|Lerp 0.0 _returnvalue Alpha))
  (bind _returnvalue_3 (Spline|GetTangentatDistanceAlongSpline _spline _returnvalue_2 "World"))
  (Transformation|SetWorldLocation (Variables|Default|GetAppaRoot) (Spline|GetLocationatDistanceAlongSpline (Variables|Default|GetSpline) _returnvalue_2 "World") false false)
  (Transformation|SetWorldRotation (Variables|Default|GetAppaRoot) (Math|Conversions|RotationFromXVector _returnvalue_3) false false)
  (return _returnvalue_3))

(fn CSetAppaonSplinePoint
  (bind _spline (Variables|Default|GetSpline))
  (bind _apparoot (Variables|Default|GetAppaRoot))
  (Transformation|SetWorldLocation _apparoot (Spline|GetLocationatSplinePoint _spline 0 "World") false false)
  (Transformation|SetWorldRotation _apparoot (Math|Conversions|RotationFromXVector (Spline|GetTangentatDistanceAlongSpline _spline 0.1 "World")) false false))

(fn DetachPlayer
  (bind _returnvalue (Game|Player|GetPlayerPawn 0))
  (Transformation|DetachFromActor (Game|Player|GetPlayerPawn 0) "KeepWorld" "KeepWorld" "KeepWorld")
  (Transformation|SetActorLocation (Game|Player|GetPlayerPawn 0) (Transformation|GetWorldLocation (Variables|Default|GetDismountPoint)) false false)
  (bind _ascharacter_movement_component (Utilities|Casting|CastToCharacterMovementComponent (Pawn|GetMovementComponent (Game|Player|GetPlayerPawn 0))))
  (Pawn|Components|CharacterMovement|SetMovementMode _ascharacter_movement_component "MOVE_Walking" 0)
  (Input|EnableInput _returnvalue (Game|GetPlayerController 0))
  (Collision|SetActorEnableCollision _returnvalue true))

(fn IsPlayerWithinThreshold
  (bind _returnvalue (Game|Player|GetPlayerPawn 0))
  (bind _appa (Variables|Default|GetAppa))
  (bind _returnvalue_2 (Transformation|GetActorLocation _returnvalue))
  (bind _returnvalue_3 (Transformation|GetWorldLocation _appa))
  (bind _returnvalue_4 (Math|Vector|Distance(Vector) _returnvalue_2 _returnvalue_3))
  (Development|PrintString (Utilities|String|ToString(Float) _returnvalue_4))
  (return (<= _returnvalue_4 (Variables|HideShow|GetDistanceThreshold))))