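; BP_AppaSpline moves a referenced target actor along a spline over a set duration when PlayTimeline is triggered.
; The construction script snaps the target to the spline's first point, facing along the tangent.
; A timeline, with play rate scaled by the inverse of Duration, interpolates distance from zero to GetSplineIndex's value.
; Each update places the target at that distance and aligns its rotation to the spline tangent.
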(event Custom|PlayTimeline
  (Components|Timeline|SetPlayRate (Variables|Default|GetMovementTimeLine) (/ 1.0 (Variables|Default|GetDuration)))
  (bind _ftrack (Timeline|MovementTimeLine PlayFromStart)
    (:Update
      (Transformation|SetActorLocation (Variables|Default|GetTargetActor) (Spline|GetLocationatDistanceAlongSpline (Variables|Default|GetSpline) (Math|Float|Lerp 0.0 (Utilities|GetSplineIndex) _ftrack) "World") false false)
      (Transformation|SetActorRotation (Variables|Default|GetTargetActor) (Math|Conversions|RotationFromXVector (Spline|GetTangentatDistanceAlongSpline (Variables|Default|GetSpline) (Math|Float|Lerp 0.0 (Utilities|GetSplineIndex) _ftrack) "World"))))))

(event EventBeginPlay)

(event Collision|EventActorBeginOverlap
  (params (OtherActor :type Actor%20Object%20Reference)))

(event EventTick
  (params (DeltaSeconds :type Float%20%28single-precision%29)))

(fn ConstructionScript
  (bind _spline (Variables|Default|GetSpline))
  (bind _targetactor (Variables|Default|GetTargetActor))
  (Transformation|SetActorLocation _targetactor (Spline|GetLocationatSplinePoint _spline 0 "World") false false)
  (Transformation|SetActorRotation _targetactor (Math|Conversions|RotationFromXVector (Spline|GetTangentatDistanceAlongSpline _spline 0.1 "World"))))