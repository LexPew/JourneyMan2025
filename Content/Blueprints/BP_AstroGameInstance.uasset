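; Game instance Blueprint that loads, restores and applies the player's AstroGameUserSettings when the game starts.
; On Init it validates the settings; the branch for an invalid settings object sets primary-display and hardware-benchmark defaults, though it calls them on that same object.
; It then re-applies display, window and frame-rate options, stores display names, overrides master, music and effects sound-class volumes, and applies the settings.
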(event EventInit
  (bind _returnvalue (Class|AstroGameUserSettings|GetAstroGameUserSettings))
  (Class|GameUserSettings|LoadSettings _returnvalue false)
  (Utilities|FlowControl|Sequence
    (:then_0
      ;[1 1 1] Validate Settings
      (bind _returnvalue_2 (Class|AstroGameUserSettings|GetAstroGameUserSettings))
      (Utilities|IsValid _returnvalue_2
        (:Is%20Valid
          (Class|GameUserSettings|ValidateSettings _returnvalue_2)
          (Class|AstroGameUserSettings|ValidateAstroUserSettings _returnvalue_2))
        (:Is%20Not%20Valid
          (bind _returnvalue_3 (Class|DisplaySettingsHelper|GetPrimaryDisplayID))
          (Class|AstroGameUserSettings|SetDisplay _returnvalue_2 _returnvalue_3)
          (Class|AstroGameUserSettings|SetLastConfirmedDisplay _returnvalue_2 _returnvalue_3)
          (bind _returnvalue_4 (Class|DisplaySettingsHelper|GetDisplayMaxResolution _returnvalue_3))
          (Class|GameUserSettings|SetScreenResolution _returnvalue_2 _returnvalue_4)
          (Class|AstroGameUserSettings|ConfirmResolution _returnvalue_2 false)
          (Class|GameUserSettings|SetBenchmarkFallbackValues _returnvalue_2)
          (Class|GameUserSettings|RunHardwareBenchmark _returnvalue_2 10 1.0 1.0)
          (Class|GameUserSettings|ApplyHardwareBenchmarkResults _returnvalue_2)
          (Class|GameUserSettings|ValidateSettings _returnvalue_2)
          (Class|AstroGameUserSettings|ValidateAstroUserSettings _returnvalue_2))))
    (:then_1
      ;[1 1 1] Display Settings
      (bind _returnvalue_5 (Class|AstroGameUserSettings|GetAstroGameUserSettings))
      (Utilities|FlowControl|Sequence
        (:then_0
          (Class|DisplaySettingsHelper|MoveGametoDisplay (Class|AstroGameUserSettings|GetDisplay _returnvalue_5)))
        (:then_1
          (Class|GameUserSettings|SetFullscreenMode _returnvalue_5 (Class|GameUserSettings|GetFullscreenMode _returnvalue_5)))
        (:then_2
          (Class|GameUserSettings|SetScreenResolution _returnvalue_5 (Class|GameUserSettings|GetScreenResolution _returnvalue_5)))
        (:then_3
          (Class|GameUserSettings|SetVSyncEnabled _returnvalue_5 (Class|GameUserSettings|IsVSyncEnabled _returnvalue_5)))
        (:then_4
          (Class|GameUserSettings|SetFrameRateLimit _returnvalue_5 (Class|GameUserSettings|GetFrameRateLimit _returnvalue_5)))
        (:then_5
          (Class|AstroGameUserSettings|SetDisplayNames _returnvalue_5 (Class|DisplaySettingsHelper|GetAllDisplayNamesPure)))))
    (:then_2
      ;[1 1 1] Sound (Control should be handled by player character)
      (bind _returnvalue_6 (Class|AstroGameUserSettings|GetAstroGameUserSettings))
      (Utilities|FlowControl|Sequence
        (:then_0
          (Audio|SetSoundMixClassOverride "/Game/Audio/MasterSoundMix.MasterSoundMix" "/Game/Audio/MasterSoundClass.MasterSoundClass" (Math|Conversions|ToFloat(Integer) (Class|AstroGameUserSettings|GetMasterVolume _returnvalue_6)) 1.0 1.0 true))
        (:then_1
          (Audio|SetSoundMixClassOverride "/Game/Audio/MusicSoundMix.MusicSoundMix" "/Game/Audio/MusicSoundClass.MusicSoundClass" (Math|Conversions|ToFloat(Integer) (Class|AstroGameUserSettings|GetMusicVolume _returnvalue_6)) 1.0 1.0 true))
        (:then_2
          (Audio|SetSoundMixClassOverride "/Game/Audio/SoundEffectSoundMix.SoundEffectSoundMix" "/Game/Audio/SoundEffectSoundClass.SoundEffectSoundClass" (Math|Conversions|ToFloat(Integer) (Class|AstroGameUserSettings|GetSoundEffectVolume _returnvalue_6)) 1.0 1.0 true))))
    (:then_3
      (Class|GameUserSettings|ApplySettings _returnvalue false))))