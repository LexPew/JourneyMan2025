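; BP_Checkpoint is a checkpoint actor that updates the player's respawn point when the player enters its sphere.
; On BeginPlay it caches the Sphere's world location and the first player pawn, cast to BP_Astro.
; When that pawn begins overlapping the Sphere, it writes the cached location into the pawn's RespawnLocation and prints a confirmation string.
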(event OnComponentBeginOverlap(Sphere)
  (params (OverlappedComponent :type Primitive%20Component%20Object%20Reference) (OtherActor :type Actor%20Object%20Reference) (OtherComp :type Primitive%20Component%20Object%20Reference) (OtherBodyIndex :type Integer) (bFromSweep :type Boolean) (SweepResult :type Hit%20Result%20Structure%20%28by%20ref%29))
  (bind _astroref (Variables|Default|GetAstroRef))
  (if (== OtherActor _astroref)
    (Variables|/Game/Blueprints/Character/BP_Astro.BP_Astro_C|SetRespawnLocation _astroref (Variables|Default|GetCheckpointLocation))
    (Development|PrintString "RespawnSet")))

(event EventBeginPlay
  (Utilities|FlowControl|Sequence
    (:then_0
      (Variables|Default|SetCheckpointLocation (Transformation|GetWorldLocation (Variables|Default|GetSphere))))
    (:then_1
      (bind _asbp_astro (Utilities|Casting|CastToBP_Astro (Game|Player|GetPlayerPawn 0)))
      (Variables|Default|SetAstroRef _asbp_astro))))

(fn ConstructionScript)