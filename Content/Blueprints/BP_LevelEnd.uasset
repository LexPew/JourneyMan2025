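; BP_LevelEnd is the level-exit trigger that stages the completion scene with the player and saved bots.
; Any Box overlap fires LevelEnd once, as the BP_Astro check is disconnected.
; It blends the view to itself, switches to WBP_LevelComplete with UI-only input and spawns Niagara fireworks.
; Bots registered through AddNPCtoArray teleport to construction-cached spawn points, consumed last-first, and Astro moves to AstroSpawn, all flagged FinishedLevel.
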(event OnComponentBeginOverlap(Box)
  (params (OverlappedComponent :type Primitive%20Component%20Object%20Reference) (OtherActor :type Actor%20Object%20Reference) (OtherComp :type Primitive%20Component%20Object%20Reference) (OtherBodyIndex :type Integer) (bFromSweep :type Boolean) (SweepResult :type Hit%20Result%20Structure%20%28by%20ref%29))
  (CallFunction|LevelEnd))

(event Custom|LevelEnd
  (bind _returnvalue (Game|Player|GetPlayerPawn 0))
  (bind _returnvalue_2 (Game|GetPlayerController 0))
  (bind _fireworkspawn1 (Variables|Default|GetFireworkSpawn1))
  (bind _fireworkspawn2 (Variables|Default|GetFireworkSpawn2))
  (bind _arrowlocations (Variables|Default|GetArrowLocations))
  (bind _returnvalue_3 (Utilities|Array|LastIndex _arrowlocations))
  (bind _returnvalue_4 (Transformation|GetWorldTransform _fireworkspawn2))
  (bind _returnvalue_5 (Transformation|GetWorldTransform _fireworkspawn1))
  (Utilities|FlowControl|DoOnce false
    (:Completed
      (Utilities|FlowControl|Sequence
        (:then_0
          (Game|Player|SetViewTargetwithBlend _returnvalue_2 self 1.0 "VTBlend_Linear" 0.0 false)
          (Input|DisableInput (Game|Player|GetPlayerPawn 0) _returnvalue_2)
          (bind _returnvalue_6 (UserInterface|CreateWidget "/Game/UI/WBP_LevelComplete.WBP_LevelComplete_C"))
          (UserInterface|Viewport|AddtoViewport _returnvalue_6 0)
          (Input|SetInputModeUIOnly _returnvalue_2 0 "DoNotLock" false)
          (Variables|/Script/Engine.PlayerController|SetbShowMouseCursor _returnvalue_2 true))
        (:then_1
          ;[1 1 1] FireworksVFX
          (Niagara|SpawnSystematLocation "/Game/FX/Fireworks_JS/NS_JS_Firework.NS_JS_Firework" (.location _returnvalue_5) "0, 0, 0" (.scale _returnvalue_5))
          (Niagara|SpawnSystematLocation "/Game/FX/Fireworks_JS/NS_JS_Firework.NS_JS_Firework" (.location _returnvalue_4) "0, 0, 0" (.scale _returnvalue_4)))
        (:then_2
          (for _array_element (Variables|Default|GetSavedBots)
            (Transformation|SetRelativeTransform (Variables|/Game/Blueprints/BP_RescuableFriendly.BP_RescuableFriendly_C|GetDefaultSceneRoot _array_element) (Math|Transform|MakeTransform (Utilities|Array|Get(acopy) _arrowlocations _returnvalue_3) "0.000000,-90.000000,0.000000" "1.000000,1.000000,1.000000") false true)
            (Variables|/Game/Blueprints/BP_RescuableFriendly.BP_RescuableFriendly_C|SetFinishedLevel? _array_element true)
            (Utilities|Array|RemoveIndex _arrowlocations _returnvalue_3))
          (bind _asbp_astro (Utilities|Casting|CastToBP_Astro _returnvalue))
          (Widget|SetVisibility (Variables|/Game/Blueprints/Character/BP_Astro.BP_Astro_C|GetAbilityWidget _asbp_astro) "Hidden")
          (Transformation|SetActorLocationAndRotation _returnvalue (Transformation|GetWorldLocation (Variables|Default|GetAstroSpawn)))
          (Variables|/Game/Blueprints/Character/BP_Astro.BP_Astro_C|SetFinishedLevel? _asbp_astro true))))))

(event Custom|AddNPCtoArray
  (params (Bot :type BP%20Rescuable%20Friendly%20Object%20Reference))
  (Utilities|Array|AddUnique (Variables|Default|GetSavedBots) Bot)
  (Development|PrintString (Utilities|GetDisplayName Bot)))

(fn ConstructionScript
  (CallFunction|SetArrowLocations))

(fn SetArrowLocations
  (Variables|Default|SetArrowLocations (Utilities|Array|MakeArray (Transformation|GetWorldLocation (Variables|Default|GetNPCSpawn1)) (Transformation|GetWorldLocation (Variables|Default|GetNPCSpawn2)) (Transformation|GetWorldLocation (Variables|Default|GetNPCSpawn3)) (Transformation|GetWorldLocation (Variables|Default|GetNPCSpawn4)) (Transformation|GetWorldLocation (Variables|Default|GetNPCSpawn5)) (Transformation|GetWorldLocation (Variables|Default|GetNPCSpawn6)))))