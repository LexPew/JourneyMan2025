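; BP_RescuableFriendly is a friendly NPC that becomes rescued when an attack hit event reaches it.
; OnAttackHit prints a debug message, sets IsRescued, calls the NPCRescued dispatcher and spawns Niagara fireworks at two component locations.
; IsAttackable always returns false, and the hit handler checks neither the attacking player nor whether the NPC is already rescued.
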(event EventBeginPlay)

(event Collision|EventActorBeginOverlap
  (params (OtherActor :type Actor%20Object%20Reference)))

(event EventTick
  (params (DeltaSeconds :type Float%20%28single-precision%29)))

(event EventOnAttackHit
  (params (AttackingPlayer :type Character%20Object%20Reference) (KnockbackStrength :type Float%20%28double-precision%29))
  (Development|PrintString "NPC Hit")
  (Utilities|FlowControl|Sequence
    (:then_0
      (Variables|Default|SetisRescued? true)
      (Default|CallNPCRescued))
    (:then_1
      (Niagara|SpawnSystematLocation "/Game/FX/Fireworks/NS_JS_Firework.NS_JS_Firework" (Transformation|GetWorldLocation (Variables|Default|GetFireworkVFX1)))
      (Niagara|SpawnSystematLocation "/Game/FX/Fireworks/NS_JS_Firework.NS_JS_Firework" (Transformation|GetWorldLocation (Variables|Default|GetFireworkVFX2))))))

(fn ConstructionScript)

(fn IsAttackable
  (return false))