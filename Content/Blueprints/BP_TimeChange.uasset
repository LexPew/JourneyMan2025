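; BP_TimeChange is a trigger volume that shifts the sky's look to a chosen time of day or weather mood when the player enters it.
; On box overlap it finds the SkyAtmosphere actor, stores its current Rayleigh scattering colour and picks a target colour from its Time setting (Day, Sunset/rise, Night or Gloomy).
; A Timeline then lerps the scattering colour from the stored value to that target.
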(event OnComponentBeginOverlap(Box)
  (params (OverlappedComponent :type Primitive%20Component%20Object%20Reference) (OtherActor :type Actor%20Object%20Reference) (OtherComp :type Primitive%20Component%20Object%20Reference) (OtherBodyIndex :type Integer) (bFromSweep :type Boolean) (SweepResult :type Hit%20Result%20Structure%20%28by%20ref%29))
  (if (== OtherActor (Game|GetPlayerCharacter 0))
    (bind _returnvalue (Actor|GetActorOfClass "/Script/Engine.SkyAtmosphere"))
    (bind _output_get (Variables|Default|SetAtmosphere%20Holder (Variables|/Script/Engine.SkyAtmosphere|GetSkyAtmosphereComponent _returnvalue)))
    (Variables|Default|SetStarting%20Colour (Variables|/Script/Engine.SkyAtmosphereComponent|GetRayleighScattering _output_get))
    (switch Utilities|FlowControl|Switch|SwitchonE_Time (Variables|Default|GetTime)
      (:NewEnumerator0
        (Variables|Default|SetDesired%20Colour "(R=0.174647,G=0.407240,B=1.000000,A=1.000000)")
        (bind _alpha (Timeline|Timeline PlayFromStart)
          (:Update
            (Class|SkyAtmosphereComponent|SetRayleighScattering (Variables|Default|GetAtmosphere%20Holder) (Math|Color|Lerp(LinearColor) (Variables|Default|GetStarting%20Colour) (Variables|Default|GetDesired%20Colour) _alpha)))))
      (:NewEnumerator1
        (Variables|Default|SetDesired%20Colour "(R=1.000000,G=0.668411,B=0.268976,A=1.000000)")
        (Timeline|Timeline PlayFromStart))
      (:NewEnumerator2
        (Variables|Default|SetDesired%20Colour "")
        (Timeline|Timeline PlayFromStart))
      (:NewEnumerator3
        (Variables|Default|SetDesired%20Colour "(R=0.390625,G=0.390625,B=0.390625,A=1.000000)")
        (Timeline|Timeline PlayFromStart)))))

(event EventBeginPlay)

(event Collision|EventActorBeginOverlap
  (params (OtherActor :type Actor%20Object%20Reference)))

(event EventTick
  (params (DeltaSeconds :type Float%20%28single-precision%29)))

(fn ConstructionScript)