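; Water wheel actor that spins up when hit by watergun actors and fires a trigger at maximum speed.
; Box overlaps with a watergun add to CurrentSpeed and destroy that actor.
; Tick applies friction-like decay, clamps the speed and feeds it to RotatingMovement's rotation rate.
; When speed exactly equals the maximum, Tick instead sets it to a hard-coded value and calls the WaterWheel event dispatcher.
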(event OnComponentBeginOverlap(Box)
  (params (OverlappedComponent :type Primitive%20Component%20Object%20Reference) (OtherActor :type Actor%20Object%20Reference) (OtherComp :type Primitive%20Component%20Object%20Reference) (OtherBodyIndex :type Integer) (bFromSweep :type Boolean) (SweepResult :type Hit%20Result%20Structure%20%28by%20ref%29))
  ;[1 1 1] Overlap/Hit Event to get initial speed
  (bind _aswatergun (Utilities|Casting|CastTowatergun OtherActor))
  (if true
    (bind _output_get (Variables|Default|SetCurrentSpeed (+ (Variables|Default|GetCurrentSpeed) (Variables|Default|GetIncreaseSpeed))))
    (Actor|DestroyActor _aswatergun)
    (Development|PrintString "Hit!")))

(event OnComponentHit(Box)
  (params (HitComponent :type Primitive%20Component%20Object%20Reference) (OtherActor :type Actor%20Object%20Reference) (OtherComp :type Primitive%20Component%20Object%20Reference) (NormalImpulse :type Vector :default "0, 0, 0") (Hit :type Hit%20Result%20Structure%20%28by%20ref%29)))

(event EventBeginPlay)

(event EventTick
  (params (DeltaSeconds :type Float%20%28single-precision%29))
  ;[1 1 1] Simulate friction and when reach to maxium speed turn on trigger
  (if (== (Variables|Default|GetCurrentSpeed) (Variables|Default|GetMaxiumSpeed))
    (Variables|Default|SetCurrentSpeed 3.6e+02)
    (Default|CallEDWaterWheel)
    (Development|PrintString "MaxiumSpeed")
    (else
      (bind _output_get (Variables|Default|SetCurrentSpeed (Math|Float|Clamp(Float) (- (Variables|Default|GetCurrentSpeed) (* (Variables|Default|GetDecreaseSpeed) (Utilities|Time|GetWorldDeltaSeconds))) 0.0 (Variables|Default|GetMaxiumSpeed))))
      (bind _output_get_2 (Variables|Default|SetRotatingMovement (Variables|Default|GetRotatingMovement)))
      (Variables|/Script/Engine.RotatingMovementComponent|SetRotationRate _output_get_2 (Math|Rotator|MakeRotator _output_get 0.0 0.0)))))

(fn ConstructionScript)