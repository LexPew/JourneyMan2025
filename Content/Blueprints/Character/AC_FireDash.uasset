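; Actor component that gives the player's BP_Astro a forward fire dash when HasFireDash is set.
; ActivateDash switches to Flying, adds forward velocity with Z zeroed, then after the duration sets Falling, or None when on Appa.
; A cooldown then clears DashActive to allow another dash.
; OnDash and OnDashReset toggle the attached Niagara fire effect and signal dash used or reset, with sound and camera shake on use.
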(event Custom|ActivateDash
  (bind _astroref (Variables|Default|GetAstroRef))
  (bind _dashvelocity (Variables|Default|GetDashVelocity))
  (bind _returnvalue (Transformation|GetActorForwardVector _astroref))
  (bind _charactermovement (Variables|/Script/Engine.Character|GetCharacterMovement _astroref))
  ;[1 1 1] Dash Logic
  (if (Variables|/Game/Blueprints/Character/BP_Astro.BP_Astro_C|GetHasFireDash _astroref)
    (if (not (Variables|Default|GetDashActive?))
      (if true
        (CallFunction|OnDash)
        (Variables|Default|SetDashActive? true)
        (Character|StopJumping _astroref)
        (Pawn|Components|CharacterMovement|SetMovementMode _charactermovement "MOVE_Flying" 0)
        (Variables|/Script/Engine.MovementComponent|SetVelocity _charactermovement (Math|Vector|MakeVector (+ (* (.x _returnvalue) _dashvelocity) (.x (Variables|/Script/Engine.MovementComponent|GetVelocity _charactermovement))) (+ (* (.y _returnvalue) _dashvelocity) (.y (Variables|/Script/Engine.MovementComponent|GetVelocity _charactermovement))) 0.0))
        (Utilities|FlowControl|Delay (Variables|Default|GetDashDuration))
        (Utilities|FlowControl|Sequence
          (:then_0
            (if (Default|GetonAppa (Variables|Default|GetAstroRef))
              (Pawn|Components|CharacterMovement|SetMovementMode _charactermovement "MOVE_None" 0)
              (else
                (Pawn|Components|CharacterMovement|SetMovementMode _charactermovement "MOVE_Falling" 0))))
          (:then_1
            (Utilities|FlowControl|Delay (Variables|Default|GetDashCooldown))
            (Variables|Default|SetDashActive? false)
            (CallFunction|OnDashReset)))))))

(event Custom|OnLanded
  (params (Hit :type Hit%20Result%20Structure%20%28by%20ref%29)))

(event Custom|OnDashReset
  (Components|Activation|SetActive (Variables|Default|GetFireDashFX) false false)
  (Default|CallDASHRESET))

(event Custom|OnDash
  ;[1 1 1] Dash Visual / Audio Logic
  (Audio|PlaySoundatLocation 0 (Transformation|GetActorLocation (Variables|Default|GetAstroRef)) "0, 0, 0" 1.0 1.0 0.0 0 0 0 0)
  ;[1 1 1] Play FOV Shake
  (CameraShakes|StartCameraShake (Game|GetPlayerCameraManager 0) "/Game/FX/FireDash_JM/BP_FireDashShake.BP_FireDashShake_C" 1.0 "CameraLocal" "0, 0, 0")
  (Components|Activation|SetActive (Variables|Default|GetFireDashFX) true false)
  (Default|CallDASHUSED))

(event EventBeginPlay
  (bind _returnvalue (Game|Player|GetPlayerPawn 0))
  ;[1 1 1] Get Ref
  (Utilities|Casting|CastToCharacter _returnvalue)
  (bind _asbp_astro (Utilities|Casting|CastToBP_Astro _returnvalue))
  ;[1 1 1] Spawn the Fire FX and attach
  (bind _output_get (Variables|Default|SetAstroRef _asbp_astro))
  (bind _returnvalue_2 (Niagara|SpawnSystemAttached "/Game/FX/FireDash_JM/NS_Fire.NS_Fire" (Variables|/Script/Engine.Actor|GetRootComponent _output_get) "None" "0, 0, 0" "0, 0, 0" "SnapToTarget" false false))
  (bind _output_get_2 (Variables|Default|SetFireDashFX _returnvalue_2))
  (Rendering|SetBoundsScale _output_get_2 5.0)
  (Default|CallDASHRESET))

(event EventTick
  (params (DeltaSeconds :type Float%20%28single-precision%29)))