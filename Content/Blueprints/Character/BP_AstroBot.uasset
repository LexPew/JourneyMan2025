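; AstroBot player character with camera-relative movement, look controls and a jump that becomes a hover when pressed again in mid-air.
; Hovering swaps gravity scale, jumps and starts a timer that applies falloff gravity; landing restores normal gravity.
; Temporary Niagara beams attached to both feet at BeginPlay show during hover and hide on jump release or landing.
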(event Custom|Hovering
  (params (IsHovering :type Boolean))
  ;[1 1 1] Hover Event
  (for _array_element (Variables|Hover|GetFootHovers)
    (Rendering|SetVisibility _array_element IsHovering false)))

(event Input|EnhancedActionEvents|EnhancedInputActionIA_Move
  (params (ActionValue :type Vector%202D%20Structure) (ElapsedSeconds :type Float%20%28double-precision%29) (TriggeredSeconds :type Float%20%28double-precision%29) (InputAction :type Input%20Action%20Object%20Reference :default "/Game/Blueprints/Character/Inputs/IA_Move.IA_Move"))
  ;[1 1 1] Add Forward / Back Movement
  (Pawn|Input|AddMovementInput (* (.y ActionValue) (Math|Vector|GetForwardVector (Variables|Default|GetCamera))) 1.0 false)
  ;[1 1 1] Add Forward / Back Movement
  (Pawn|Input|AddMovementInput (* (.x ActionValue) (Math|Vector|GetRightVector (Variables|Default|GetCamera))) 1.0 false))

(event Input|EnhancedActionEvents|EnhancedInputActionIA_Look
  (params (ActionValue :type Vector%202D%20Structure) (ElapsedSeconds :type Float%20%28double-precision%29) (TriggeredSeconds :type Float%20%28double-precision%29) (InputAction :type Input%20Action%20Object%20Reference :default "/Game/Blueprints/Character/Inputs/IA_Look.IA_Look"))
  ;[1 1 1] Camera Controls
  (Pawn|Input|AddControllerPitchInput (.y ActionValue))
  (Pawn|Input|AddControllerYawInput (.x ActionValue)))

(event Input|EnhancedActionEvents|EnhancedInputActionIA_Jump
  (params (ActionValue :type Boolean) (ElapsedSeconds :type Float%20%28double-precision%29) (TriggeredSeconds :type Float%20%28double-precision%29) (InputAction :type Input%20Action%20Object%20Reference :default "/Game/Blueprints/Character/Inputs/IA_Jump.IA_Jump"))
  ;[1 1 1] Jumping & Hover Movement
  (:Started
    (if (AI|Components|NavMovement|IsFalling (Variables|Character|GetCharacterMovement))
      (CallFunction|TryHover)
      (else
        (Character|Jump))))
  (:Completed
    (CallFunction|Hovering false)
    (Character|StopJumping)))

(event EventBeginPlay
  ;[1 1 1] Adds the Input Mapping Context
  (bind _asplayer_controller (Utilities|Casting|CastToPlayerController (Pawn|GetController)))
  (Utilities|IsValid (PlayerController|LocalPlayerSubsystems|GetEnhancedInputLocalPlayerSubsystem _asplayer_controller)
    (:Is%20Valid
      (Input|AddMappingContext (PlayerController|LocalPlayerSubsystems|GetEnhancedInputLocalPlayerSubsystem _asplayer_controller) "/Game/Blueprints/Character/Inputs/IMC_Character.IMC_Character" 0 "(bIgnoreAllPressedKeysUntilRelease=True,bForceImmediately=False,bNotifyUserSettings=False)")
      ;[1 1 1] Adds The Temporary Hover Beams
      (CallFunction|AttachHoverBeamTemp))))

(event Collision|EventActorBeginOverlap
  (params (OtherActor :type Actor%20Object%20Reference)))

(event EventTick
  (params (DeltaSeconds :type Float%20%28single-precision%29)))

(event EventOnLanded
  (params (Hit :type Hit%20Result%20Structure%20%28by%20ref%29))
  ;[1 1 1] Reset Gravity On Landing And Reset Hover Event
  (CallFunction|Hovering false)
  (CallFunction|ResetGravity))

(fn ConstructionScript)

(fn FallGravity
  (Variables|/Script/Engine.CharacterMovementComponent|SetGravityScale (Variables|Character|GetCharacterMovement) (Variables|Hover|GetFalloffGravity)))

(fn ResetGravity
  (Variables|/Script/Engine.CharacterMovementComponent|SetGravityScale (Variables|Character|GetCharacterMovement) 1.0)
  (Variables|Hover|SetIsHovering false))

(fn AttachHoverBeamTemp
  (bind _mesh (Variables|Character|GetMesh))
  (bind _returnvalue (Niagara|SpawnSystemAttached "/Game/FX/NS_HoverBeam.NS_HoverBeam" _mesh "foot_l" "0, 0, 0" "0, 0, 0" "KeepRelativeOffset" false))
  (Utilities|Array|Add (Variables|Hover|GetFootHovers) _returnvalue)
  (bind _returnvalue_2 (Niagara|SpawnSystemAttached "/Game/FX/NS_HoverBeam.NS_HoverBeam" _mesh "foot_r" "0, 0, 0" "0.000000,-180.000000,0.000000" "KeepRelativeOffset" false))
  (Utilities|Array|Add (Variables|Hover|GetFootHovers) _returnvalue_2)
  (CallFunction|Hovering false))

(fn TryHover
  (if (not (and (Variables|Hover|GetIsHovering) (== (Variables|Default|GetJumpCurrentCount) 0)))
    (Variables|/Script/Engine.CharacterMovementComponent|SetGravityScale (Variables|Character|GetCharacterMovement) (Variables|Hover|GetHoveringGravityScale))
    (Character|Jump)
    (Utilities|Time|SetTimerbyFunctionName 0 "FallGravity" (Variables|Hover|GetTotalHoverTime))
    (Variables|Hover|SetIsHovering true)
    (CallFunction|Hovering true)))