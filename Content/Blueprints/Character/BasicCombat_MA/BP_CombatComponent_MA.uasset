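; Melee combat component for BP_Astro that turns attack input into montage attacks with hitbox checks.
; IA_Attack plays the AM_Attacks section named by the current ComboChain entry, gated until the montage completes, with held input throttled.
; Box hitboxes, offset relative to the owner, are debug-drawn and overlap-tested once, sending BPI_Attackable hits with fixed knockback.
; Sphere and capsule hitboxes are unimplemented, and the HitDetection counter event is not called by the attack flow.
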(event Custom|HitDetection
  (params (Duration :type Float%20%28double-precision%29))
  (Math|Float|IncrementFloat (Variables|Default|GetCounter)
    (:%20%20
      (if (< (Variables|Default|GetCounter) Duration)
        (CallFunction|HitDetection Duration)
        (else
          (Variables|Default|SetCounter 0.0))))))

(event Input|EnhancedActionEvents|EnhancedInputActionIA_Attack
  (params (ActionValue :type Boolean) (ElapsedSeconds :type Float%20%28double-precision%29) (TriggeredSeconds :type Float%20%28double-precision%29) (InputAction :type Input%20Action%20Object%20Reference :default "/Game/Blueprints/Character/Inputs/IA_Attack.IA_Attack"))
  (bind _returnvalue (Components|GetOwner))
  (bind _combochain (Variables|Default|GetComboChain))
  (bind _currentattackindex (Variables|Default|GetCurrentAttackIndex))
  (bind _output (Utilities|Array|Get(acopy) _combochain _currentattackindex))
  (bind (_attackanimation _damage _attackduration _hitboxshape _hitboxsize _hitboxoffset _hitboxrotation) (Utilities|Struct|BreakAttackData _output))
  (bind (_x _y _z) (Math|Vector|BreakVector _hitboxoffset))
  (bind (_returnvalue_2 _returnvalue2) (Utilities|NewMacro _returnvalue _returnvalue _returnvalue _returnvalue _x _y _z _hitboxrotation))
  (:Triggered
    (bind _output_get (Variables|Default|SetTimeSinceLastTrigger (- ElapsedSeconds (Variables|Default|GetLastTriggerTime))))
    (if (>= _output_get 0.5)
      (Variables|Default|SetLastTriggerTime ElapsedSeconds)
      (Class|ACCombatComponent|StartAttack :!label _label)
      (if (Variables|Default|GetbAllowNextAttack)
        (Animation|Montage|PlayMontage (Variables|/Script/Engine.Character|GetMesh (Variables|Default|GetAstroRef)) "/Game/Characters/Astrobot/Animations/AnimMontages/AM_Attacks.AM_Attacks" 1.0 0.0 (Utilities|String|StringToName (Utilities|String|EnumtoString _attackanimation))
          (:then
            (Variables|Default|SetbAllowNextAttack false)
            (switch Utilities|FlowControl|Switch|SwitchonEHitboxShape _hitboxshape
              (:Box
                (Rendering|Debug|DrawDebugBox :Center _returnvalue_2 :Extent _hitboxsize :Rotation _returnvalue2)
                (bind _outactors (Collision|BoxOverlapActors _returnvalue_2 _hitboxsize (Utilities|Array|MakeArray "ObjectTypeQuery3" "ObjectTypeQuery6" "ObjectTypeQuery4") 0 :!class /Script/Engine.KismetSystemLibrary))
                (for _array_element _outactors
                  (if (Utilities|DoesObjectImplementInterface _array_element "/Game/Blueprints/Character/BasicCombat_MA/BPI_Attackable.BPI_Attackable_C")
                    (Class|BPIAttackable|OnAttackHit(Message) _array_element (Variables|Default|GetAstroRef) 1e+04))))))
          (:OnCompleted
            (Variables|Default|SetbAllowNextAttack true))))))
  (:Started
    (goto _label)))

(event EventBeginPlay
  (bind _asbp_astro (Utilities|Casting|CastToBP_Astro (Components|GetOwner)))
  (Variables|Default|SetAstroRef _asbp_astro))