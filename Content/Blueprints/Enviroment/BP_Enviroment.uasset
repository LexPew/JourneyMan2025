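; BP_Enviroment is a trigger volume that applies local atmosphere (fog, Niagara effect, 2D sound, directional light intensity) while the player is inside its box.
; On player entry it reveals the effects and a timeline eases the light and fog to target values.
; On exit it stops the sound, restores the cached light intensity and fades the fog before hiding everything.
; Empty Overlapped and StopOverlap events serve as hooks.
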(event OnComponentBeginOverlap(Box)
  (params (OverlappedComponent :type Primitive%20Component%20Object%20Reference) (OtherActor :type Actor%20Object%20Reference) (OtherComp :type Primitive%20Component%20Object%20Reference) (OtherBodyIndex :type Integer) (bFromSweep :type Boolean) (SweepResult :type Hit%20Result%20Structure%20%28by%20ref%29))
  (bind _niagra_system (Variables|Default|GetNiagra_System))
  (CallFunction|Overlapped)
  (if (CallFunction|IsPlayer OtherActor)
    (CallFunction|SetVis true)
    (bind _returnvalue (Audio|SpawnSound2D (Variables|Default|GetEnviroment_Sound) 1.0 1.0 0.0 0))
    (Variables|Default|SetSound _returnvalue)
    ;[1 1 1] Handle Intro
    (Components|Activation|Activate _niagra_system false)
    (Rendering|SetBoundsScale _niagra_system (Variables|Default|GetBounds_Scale))
    (bind _returnvalue_2 (Actor|GetActorOfClass "/Script/Engine.DirectionalLight"))
    (bind _output_get (Variables|Default|SetDir_Light _returnvalue_2))
    (Variables|Default|SetCached_Intensity (Variables|/Script/Engine.LightComponentBase|GetIntensity (Variables|/Script/Engine.Light|GetLightComponent _output_get)))
    (bind _ftrack (Timeline|LerpIn PlayFromStart)
      (:Update
        (Rendering|Components|Light|SetIntensity (Variables|/Script/Engine.Light|GetLightComponent (Variables|Default|GetDir_Light)) (Math|Float|Lerp (Variables|/Script/Engine.LightComponentBase|GetIntensity (Variables|/Script/Engine.Light|GetLightComponent (Variables|Default|GetDir_Light))) (Variables|Default|GetFinal_Light_Int) _ftrack))
        (Class|LocalFogVolumeComponent|SetHeightFogExtinction (Variables|Default|GetLocalFogVolume) (Math|Float|Lerp 0.0 (Variables|Default|GetFinal_Fog_Int) _ftrack))))))

(event OnComponentEndOverlap(Box)
  (params (OverlappedComponent :type Primitive%20Component%20Object%20Reference) (OtherActor :type Actor%20Object%20Reference) (OtherComp :type Primitive%20Component%20Object%20Reference) (OtherBodyIndex :type Integer))
  (bind _sound (Variables|Default|GetSound))
  ;[1 1 1] Deact
  (if (CallFunction|IsPlayer OtherActor)
    (CallFunction|StopOverlap)
    (Utilities|IsValid _sound
      (:Is%20Valid
        (Audio|Components|Audio|Stop _sound))
      (:Is%20Not%20Valid
        _))
    (CallFunction|ResetL)
    (bind _ftrack (Timeline|Timeline PlayFromStart)
      (:Update
        (Class|LocalFogVolumeComponent|SetHeightFogExtinction (Variables|Default|GetLocalFogVolume) (Math|Float|Lerp (Variables|Default|GetFinal_Fog_Int) 0.0 _ftrack)))
      (:Finished
        (Components|Activation|Deactivate (Variables|Default|GetNiagra_System))
        (CallFunction|SetVis false)))))

(event Custom|Overlapped)

(event Custom|StopOverlap)

(event Custom|ResetL
  (bind _dir_light (Variables|Default|GetDir_Light))
  (bind _lightcomponent (Variables|/Script/Engine.Light|GetLightComponent _dir_light))
  (bind _newtrack_0 (Timeline|ResetTimeline PlayFromStart)
    (:Update
      (Rendering|Components|Light|SetIntensity _lightcomponent (Math|Float|Lerp (Variables|/Script/Engine.LightComponentBase|GetIntensity _lightcomponent) (Variables|Default|GetCached_Intensity) _newtrack_0)))))

(event EventBeginPlay
  (CallFunction|SetVis false))

(fn ConstructionScript)

(fn SetVis
  (params (Visible :type Boolean))
  (Rendering|SetVisibility (Variables|Default|GetLocalFogVolume) Visible false)
  (Rendering|SetVisibility (Variables|Default|GetNiagra_System) Visible false))

(fn IsPlayer
  (params (OtherActor :type Actor%20Object%20Reference))
  (return (== OtherActor (Game|Player|GetPlayerPawn 0))))