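; BP_Enviroment_Rainy is a rainy environment Blueprint that shows or hides its NGCloud effect component in response to overlap events.
; NGCloud is hidden on BeginPlay, after the parent's logic runs.
; Overlapped makes the cloud visible, while StopOverlap hides and deactivates it, each with a debug print.
; Overlapped only changes visibility and does not reactivate the component after StopOverlap deactivates it.
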(event EventBeginPlay
  (|CallParentFunction)
  (Rendering|SetVisibility (Variables|Default|GetNG_Cloud) false false))

(event Collision|EventActorBeginOverlap
  (params (OtherActor :type Actor%20Object%20Reference)))

(event EventTick
  (params (DeltaSeconds :type Float%20%28single-precision%29)))

(event EventOverlapped
  (Development|PrintString "Overlap")
  (Rendering|SetVisibility (Variables|Default|GetNG_Cloud) true false))

(event EventStopOverlap
  (Development|PrintString "StopLap")
  (Rendering|SetVisibility (Variables|Default|GetNG_Cloud) false false)
  (Components|Activation|Deactivate (Variables|Default|GetNG_Cloud)))

(fn ConstructionScript
  (|CallParentFunction))