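; Player controller for the main menu that shows the menu UI and reacts to player input.
; On BeginPlay it adds the main menu Enhanced Input mapping context, shows the mouse cursor with permanent viewport capture, and creates and displays WBP_MainMenu.
; When the IA_Any input action starts, it tells the stored menu widget to show the saves menu.
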(event Input|EnhancedActionEvents|EnhancedInputActionIA_Any
  (params (ActionValue :type Boolean) (ElapsedSeconds :type Float%20%28double-precision%29) (TriggeredSeconds :type Float%20%28double-precision%29) (InputAction :type Input%20Action%20Object%20Reference :default "/Game/Input/InputActions/IA_Any.IA_Any"))
  (:Started
    (Default|ShowSavesMenu (Variables|Default|GetMainMenuWidget))))

(event EventBeginPlay
  (bind _self self)
  (Input|AddMappingContext (PlayerController|LocalPlayerSubsystems|GetEnhancedInputLocalPlayerSubsystem self) "/Game/Input/IMC_MainMenu.IMC_MainMenu" 0 "(bIgnoreAllPressedKeysUntilRelease=True,bForceImmediately=False,bNotifyUserSettings=False)")
  (Variables|/Script/Engine.PlayerController|SetbShowMouseCursor _self true)
  (Class|GameplayStatics|SetViewportMouseCaptureMode "CapturePermanently")
  (bind _returnvalue (UserInterface|CreateWidget "/Game/UI/WBP_MainMenu.WBP_MainMenu_C" _self))
  (bind _output_get (Variables|Default|SetMainMenuWidget _returnvalue))
  (UserInterface|Viewport|AddtoViewport _output_get 0))

(event EventTick
  (params (DeltaSeconds :type Float%20%28single-precision%29)))

(fn ConstructionScript)