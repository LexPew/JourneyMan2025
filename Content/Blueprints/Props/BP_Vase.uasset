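; BP_Vase is a breakable vase prop that shatters when BP_Astro hits it with an attack.
; An intact static mesh is shown while the Geometry Collection stays hidden and inert from BeginPlay.
; OnAttackHit from Astro swaps to the physics-simulated collection, crumbles its cluster, plays a random-pitched break sound and sets a short lifespan.
; IsAttackable always returns false.
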(event EventBeginPlay
  (CallFunction|DisableGC))

(event Collision|EventActorBeginOverlap
  (params (OtherActor :type Actor%20Object%20Reference)))

(event EventTick
  (params (DeltaSeconds :type Float%20%28single-precision%29)))

(event EventOnAttackHit
  (params (AttackingPlayer :type Character%20Object%20Reference) (KnockbackStrength :type Float%20%28double-precision%29))
  (Development|PrintString "Hello")
  (if (.bSuccess (Utilities|Casting|CastToBP_Astro AttackingPlayer))
    (CallFunction|EnableGC)))

(fn ConstructionScript)

(fn DisableGC
  (Rendering|SetVisibility (Variables|Default|GetGC_Vase) false false)
  (Physics|SetSimulatePhysics (Variables|Default|GetGC_Vase) false)
  (Collision|SetCollisionEnabled (Variables|Default|GetGC_Vase) "NoCollision"))

(fn EnableGC
  ;[1 1 1] SM
  (Rendering|SetVisibility (Variables|Default|GetStaticMesh) false false)
  (Collision|SetCollisionEnabled (Variables|Default|GetStaticMesh) "NoCollision")
  ;[1 1 1] Vase GC
  (Rendering|SetVisibility (Variables|Default|GetGC_Vase) true false)
  (Physics|SetSimulatePhysics (Variables|Default|GetGC_Vase) true)
  (Collision|SetCollisionEnabled (Variables|Default|GetGC_Vase) "PhysicsOnly")
  (Class|GeometryCollectionComponent|CrumbleCluster (Variables|Default|GetGC_Vase))
  (CallFunction|PlayAudio)
  (Actor|SetLifeSpan 2.0))

(fn PlayAudio
  (Audio|PlaySoundatLocation (Variables|Default|GetBreak_Sound) (Transformation|GetActorLocation) "0, 0, 0" (Variables|Default|GetVol_Multi) (Math|Random|RandomFloatinRange 0.65 1.2) 0.0 0 0 0 0))

(fn IsAttackable
  (return false))