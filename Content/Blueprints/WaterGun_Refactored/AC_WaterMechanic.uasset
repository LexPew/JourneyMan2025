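; AC_WaterMechanic is a component that provides the firing action for a water gun.
; Initialize caches the camera and spawn point references it is given.
; FireWaterGun spawns a BP_WaterCollider just ahead of the spawn point along the camera's forward vector, matching the camera's rotation and ignoring collisions at spawn.
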(event Custom|Fire%20Water%20Gun
  (Game|SpawnActorfromClass "/Game/Blueprints/WaterGun_Refactored/BP_WaterCollider.BP_WaterCollider_C" (Math|Transform|MakeTransform (+ (Transformation|GetWorldLocation (Variables|Default|GetSpawnPoint)) (Math|Vector|GetForwardVector (Variables|Default|GetCamera))) (Transformation|GetWorldRotation (Variables|Default|GetCamera)) "1.000000,1.000000,1.000000") "AlwaysSpawn" "MultiplyWithRoot" 0 0))

(event EventBeginPlay)

(event EventTick
  (params (DeltaSeconds :type Float%20%28single-precision%29)))

(fn Initialize
  (params (P_Camera :type Camera%20Component%20Object%20Reference) (P_SpawnPosition :type Arrow%20Component%20Object%20Reference))
  (Variables|Default|SetSpawnPoint P_SpawnPosition)
  (Variables|Default|SetCamera P_Camera))