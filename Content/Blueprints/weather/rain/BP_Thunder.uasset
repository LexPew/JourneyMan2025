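; Lightning and thunder actor that produces repeating strikes around the player once startstrike is triggered.
; startstrike loops on a random delay, calling Strike and playing the thunder sound.
; Strike relocates the actor to a random raised spot ahead of the player's view, yawed toward the player, then runs a timeline driving the bolt material's Y and Emission parameters.
; An exposure flash through the post-process volume is present but disconnected.
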(event Custom|Strike
  (|Re-locate
    (:OutputPin
      (bind (_direction _emission _y) (Timeline|Timeline PlayFromStart)
        (:Update
          (Rendering|Material|SetScalarParameterValueonMaterials (Variables|Default|GetThunder) "Y" _y)
          (Rendering|Material|SetScalarParameterValueonMaterials (Variables|Default|GetThunder) "Emission" (* _emission 1e+01)))))))

(event Custom|start%20strike
  (Utilities|FlowControl|Delay (Math|Random|RandomFloatinRange 9.0 15.0) :!label _label)
  (CallFunction|Strike)
  (Audio|Components|Audio|Play (Variables|Default|GetSound_Thunder) 0.0)
  (goto _label))

(event EventBeginPlay)

(fn ConstructionScript)