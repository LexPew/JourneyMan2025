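; BP_HoverBeam is an effect actor whose beam length adjusts to the distance of the surface it points at.
; Every Tick, CalculateLength line-traces on the Visibility channel along the Arrow component's forward vector, up to MaxRayDistance.
; On a hit, a value derived from the hit distance feeds the Z of the Beam effect's BeamHeight vector variable; a miss leaves it unchanged.
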(event EventBeginPlay)

(event Collision|EventActorBeginOverlap
  (params (OtherActor :type Actor%20Object%20Reference)))

(event EventTick
  (params (DeltaSeconds :type Float%20%28single-precision%29))
  (CallFunction|CalculateLength))

(fn ConstructionScript)

(fn CalculateLength
  (bind _arrow (Variables|Default|GetArrow))
  (bind _returnvalue (Transformation|GetWorldLocation _arrow))
  (bind (_outhit _returnvalue_2) (Collision|LineTraceByChannel _returnvalue (+ _returnvalue (* (Math|Vector|GetForwardVector _arrow) (Variables|Default|GetMaxRayDistance))) "TraceTypeQuery1" false 0 "None"))
  (if _returnvalue_2
    (bind _result (Math|Float|NegateFloat (Math|Vector|VectorLength (- (.location _outhit) (Transformation|GetWorldLocation (Variables|Default|GetArrow)))))
      (:%20%20
        (Niagara|SetNiagaraVariable(Vector3) (Variables|Default|GetBeam) "BeamHeight" (Math|Vector|MakeVector 0.0 0.0 _result))))))