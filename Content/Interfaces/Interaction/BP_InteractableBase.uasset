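; BP_InteractableBase is a base Blueprint for interactables that highlights meshes through Render Custom Depth.
; StartOverlap enables custom depth on every mesh in MeshesToHighlight when ShouldHighlight is true, and otherwise calls EndOverlap, which disables it.
; Child Blueprints are meant to supply their meshes through SetMeshesToHighlight, shown here only as an unconnected example call.
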(event EventStartOverlap
  ;[1 0.8435 0] Highlight Material
  (if (Variables|Default|GetShouldHighlight?)
    (for _array_element (Variables|Default|GetMeshesToHighlight)
      (Rendering|SetRenderCustomDepth _array_element true))
    (else
      (CallFunction|EndOverlap))))

(event EventEndOverlap
  ;[1 0.8435 0] Highlight Material
  (for _array_element (Variables|Default|GetMeshesToHighlight)
    (Rendering|SetRenderCustomDepth _array_element false)))

(fn ConstructionScript)

(fn SetMeshestoHighlight
  (params (Meshes :type Array%20of%20Primitive%20Component%20Object%20References))
  (Variables|Default|SetMeshesToHighlight Meshes))