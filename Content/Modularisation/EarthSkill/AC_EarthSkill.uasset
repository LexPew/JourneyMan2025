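; Earth skill actor component that lets its owner pick up, carry, then throw or drop physics objects marked with AC_Carriable.
; StartHolding traces from the spring arm along camera forward, then grabs the hit actor's mesh with the owner's physics handle at HoldLocation.
; Holding updates the handle target and accumulates hold time.
; StopHolding throws along camera forward with time-scaled impulse after a long hold, otherwise calls DropObject to restore physics.
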(event Custom|StartHolding
  (params (Hold%20Location :type Arrow%20Component%20Object%20Reference))
  (bind _springarm (Variables|Default|GetSpringArm))
  (bind _returnvalue (Transformation|GetWorldLocation _springarm))
  (Variables|Default|SetHoldLocation Hold%20Location)
  (bind (_outhit _returnvalue_2) (Collision|LineTraceByChannel _returnvalue (+ _returnvalue (* (Math|Vector|GetForwardVector (Transformation|GetWorldRotation (Variables|Default|GetCamera))) 2e+02)) "TraceTypeQuery1" false 0 "ForDuration"))
  (if _returnvalue_2
    (Utilities|IsValid (Actor|GetComponentbyClass (.HitActor (Collision|BreakHitResult _outhit)) "/Game/Blueprints/AC_Carriable.AC_Carriable_C")
      (:Is%20Valid
        (Development|PrintString "PickUp Succeed")
        (Variables|Default|SetCarriedObj (Actor|GetComponentbyClass (.HitActor (Collision|BreakHitResult _outhit)) "/Script/Engine.StaticMeshComponent"))
        (Collision|SetCollisionEnabled (Actor|GetComponentbyClass (.HitActor (Collision|BreakHitResult _outhit)) "/Script/Engine.StaticMeshComponent") "PhysicsOnly")
        (Transformation|SetActorLocation (.HitActor (Collision|BreakHitResult _outhit)) (Transformation|GetWorldLocation (Variables|Default|GetHoldLocation)) false false)
        (Physics|Components|PhysicsHandle|GrabComponentatLocationwithRotation (Variables|Default|GetPhysicsHandle) (Variables|Default|GetCarriedObj) "None" (Transformation|GetWorldLocation (Variables|Default|GetHoldLocation)) (Math|Rotator|MakeRotator 0.0 0.0 0.0))
        (Class|PrimitiveComponent|SetAngularDamping (Variables|Default|GetCarriedObj) 5e+03))
      (:Is%20Not%20Valid
        (Development|PrintString "PickUp Failed" :!label _label)))
    (else
      (goto _label))))

(event Custom|Holding
  (bind _holdlocation (Variables|Default|GetHoldLocation))
  (if true
    (Class|PhysicsHandleComponent|SetTargetLocationandRotation (Variables|Default|GetPhysicsHandle) (Transformation|GetWorldLocation _holdlocation) (Math|Rotator|MakeRotator 0.0 0.0 (.yaw (Transformation|GetWorldRotation _holdlocation))))
    (Variables|Default|SetObjHoldTime (+ (Variables|Default|GetObjHoldTime) 0.1))))

(event Custom|StopHolding
  (params (Triggered%20Seconds :type Float%20%28double-precision%29))
  (if (Utilities|IsValid (Variables|Default|GetCarriedObj))
    (if (> Triggered%20Seconds 2.0)
      (Physics|Components|PhysicsHandle|ReleaseComponent (Variables|Default|GetPhysicsHandle))
      (Collision|SetCollisionEnabled (Actor|GetComponentbyClass (.HitActor (Collision|BreakHitResult (stale Custom|StartHolding _outhit))) "/Script/Engine.StaticMeshComponent") "QueryAndPhysics")
      (Physics|AddImpulse (Actor|GetComponentbyClass (.HitActor (Collision|BreakHitResult (stale Custom|StartHolding _outhit))) "/Script/Engine.StaticMeshComponent") (* (Math|Vector|GetForwardVector (Variables|Default|GetCamera)) (* (Variables|Default|GetObjHoldTime) 1e+04)) "None" false)
      (Variables|Default|SetObjHoldTime 1.0)
      (else
        (CallFunction|DropObject (Variables|Default|GetCarriedObj))))))

(event EventBeginPlay
  (bind _returnvalue (Components|GetOwner))
  (bind _returnvalue_2 (Actor|GetComponentbyClass _returnvalue "/Script/Engine.PhysicsHandleComponent"))
  (bind _returnvalue_3 (Actor|GetComponentbyClass _returnvalue "/Script/Engine.CameraComponent"))
  (bind _returnvalue_4 (Actor|GetComponentbyClass _returnvalue "/Script/Engine.SpringArmComponent"))
  (Utilities|IsValid _returnvalue_3
    (:Is%20Valid
      (Variables|Default|SetCamera _returnvalue_3))
    (:Is%20Not%20Valid
      (Development|PrintString "Camera Not Found")))
  (Utilities|IsValid _returnvalue_4
    (:Is%20Valid
      (Variables|Default|SetSpringArm _returnvalue_4))
    (:Is%20Not%20Valid
      (Development|PrintString "Spring Arm not found")))
  (Utilities|IsValid _returnvalue_2
    (:Is%20Valid
      (Variables|Default|SetPhysicsHandle _returnvalue_2))
    (:Is%20Not%20Valid
      (Development|PrintString "Physics Handle Not Found"))))

(event EventTick
  (params (DeltaSeconds :type Float%20%28single-precision%29)))

(fn DropObject
  (params (CarriedObj :type Static%20Mesh%20Component%20Object%20Reference))
  (Physics|Components|PhysicsHandle|ReleaseComponent (Variables|Default|GetPhysicsHandle))
  (Class|PrimitiveComponent|WakeRigidBody CarriedObj "None")
  (Physics|SetEnableGravity CarriedObj true)
  (Class|PrimitiveComponent|SetAngularDamping CarriedObj 0.0)
  (Collision|SetCollisionEnabled CarriedObj "QueryAndPhysics")
  (Variables|Default|SetCarriedObj 0))