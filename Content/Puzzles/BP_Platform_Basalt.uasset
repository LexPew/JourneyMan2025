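; BP_Platform_Basalt is a puzzle platform that drops away when a Character touches it, then returns.
; A sphere overlap plays the DropDown sequence, then delays disable collision and hide the actor, later restore both, and play RiseUp.
; A DoOnce blocks retriggers until the cycle ends, but it precedes the Character cast, so any other overlapping actor consumes it without a reset.
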(event OnComponentBeginOverlap(Sphere)
  (params (OverlappedComponent :type Primitive%20Component%20Object%20Reference) (OtherActor :type Actor%20Object%20Reference) (OtherComp :type Primitive%20Component%20Object%20Reference) (OtherBodyIndex :type Integer) (bFromSweep :type Boolean) (SweepResult :type Hit%20Result%20Structure%20%28by%20ref%29))
  (Utilities|FlowControl|DoOnce false :!label _label
    (:Completed
      (Utilities|Casting|CastToCharacter OtherActor)
      (Class|ActorSequenceComponent|PlaySequence (Variables|Default|GetDrop%20Down))
      (Utilities|FlowControl|Delay 1.0)
      (Collision|SetActorEnableCollision false)
      (Rendering|SetActorHiddenInGame true)
      (Utilities|FlowControl|Delay 7.5)
      (Collision|SetActorEnableCollision true)
      (Rendering|SetActorHiddenInGame false)
      (Utilities|FlowControl|Delay 1.0)
      (Class|ActorSequenceComponent|PlaySequence (Variables|Default|GetRise%20Up))
      (Utilities|FlowControl|Delay 2.0)
      (goto _label Reset))))

(event EventBeginPlay)

(event Collision|EventActorBeginOverlap
  (params (OtherActor :type Actor%20Object%20Reference)))

(event EventTick
  (params (DeltaSeconds :type Float%20%28single-precision%29)))

(fn ConstructionScript)