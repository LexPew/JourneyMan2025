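; Interactable puzzle rock platform that slides along its relative X axis while the interaction is held.
; A timeline lerps the mesh from its start location to an offset goal, with its play rate set from TimeToPull.
; Ending the interaction early reverses the timeline, sliding the platform back.
; Reaching the goal within a small tolerance marks it finished, which blocks further interaction and disables highlighting.
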(event EventInteract
  (bind _startlocation (Variables|Default|GetStartLocation))
  (bind _goallocation (Variables|Default|GetGoalLocation))
  (if (not (Variables|Default|GetFinished))
    (bind _rockpullprogress (Timeline|PullRock Play)
      (:Update
        (Transformation|SetRelativeLocation (Variables|Default|GetPlatformMesh) (Math|Vector|MakeVector (Math|Float|Lerp (.x _startlocation) (.X (Math|Vector|BreakVector _goallocation)) _rockpullprogress) (.y _startlocation) (.z _startlocation)) false false))
      (:Finished
        (if (Utilities|Operators|EqualEqual (.location (Transformation|GetRelativeTransform (Variables|Default|GetPlatformMesh))) _goallocation 5.0)
          (Variables|Default|SetFinished true)
          (Variables|Default|SetShouldHighlight? false))))))

(event EventBeginPlay
  (bind _platformmesh (Variables|Default|GetPlatformMesh))
  (bind _returnvalue (Transformation|GetRelativeTransform _platformmesh))
  (bind (_x _y _z) (Math|Vector|BreakVector (.location _returnvalue)))
  (CallFunction|SetMeshestoHighlight (Utilities|Array|MakeArray (Variables|Default|GetPlatformMesh)))
  (Components|Timeline|SetPlayRate (Variables|Default|GetPullRock) (Variables|Default|GetTimeToPull))
  (Variables|Default|SetStartLocation (.location _returnvalue))
  (Variables|Default|SetGoalLocation (Math|Vector|MakeVector (+ _x (Variables|Default|GetValueToAdd)) _y _z)))

(event EventEndInteract
  (bind _startlocation (Variables|Default|GetStartLocation))
  (bind _goallocation (Variables|Default|GetGoalLocation))
  (if (not (Variables|Default|GetFinished))
    (Utilities|FlowControl|Sequence
      (:then_0
        (bind _rockpullprogress (Timeline|PullRock Stop)
          (:Update
            (Transformation|SetRelativeLocation (Variables|Default|GetPlatformMesh) (Math|Vector|MakeVector (Math|Float|Lerp (.x _startlocation) (.X (Math|Vector|BreakVector _goallocation)) _rockpullprogress) (.y _startlocation) (.z _startlocation)) false false))
          (:Finished
            (if (Utilities|Operators|EqualEqual (.location (Transformation|GetRelativeTransform (Variables|Default|GetPlatformMesh))) _goallocation 5.0)
              (Variables|Default|SetFinished true)
              (Variables|Default|SetShouldHighlight? false)))))
      (:then_1
        (Timeline|PullRock Reverse)))))

(fn ConstructionScript)