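; BP_VideoPlayer is a trigger actor that shows a tutorial video when something overlaps its Box.
; On BeginPlay it creates a WB_TutorialUI widget, adds it to the viewport and keeps it hidden.
; Any overlap reveals the widget and passes it the actor's media player, video material and media source for playback; a BP_Astro filter exists but is disconnected, and nothing here hides the widget again.
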(event OnComponentBeginOverlap(Box)
  (params (OverlappedComponent :type Primitive%20Component%20Object%20Reference) (OtherActor :type Actor%20Object%20Reference) (OtherComp :type Primitive%20Component%20Object%20Reference) (OtherBodyIndex :type Integer) (bFromSweep :type Boolean) (SweepResult :type Hit%20Result%20Structure%20%28by%20ref%29))
  (bind _tutorialui (Variables|Default|GetTutorialUI))
  (Widget|SetVisibility _tutorialui "Visible")
  (Default|PlayVideo _tutorialui (Variables|Default|GetMediaPlayer) (Variables|Default|GetVideo%20Material) (Variables|Default|GetMediaSource)))

(event EventBeginPlay
  (bind _returnvalue (UserInterface|CreateWidget "/Game/VideoUI/WB_TutorialUI.WB_TutorialUI_C"))
  (UserInterface|Viewport|AddtoViewport _returnvalue 0)
  (bind _output_get (Variables|Default|SetTutorialUI _returnvalue))
  (Widget|SetVisibility _output_get "Hidden"))

(fn ConstructionScript)